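; Player state Blueprint that hosts the player's ability system, character attribute and gameplay tag components, exposing them through accessor functions.
; InitCharacterData binds to inventory and hotbar weight-change events, which write their combined weight into the base Weight attribute.
; On authority, BeginPlay applies a test weight bonus effect and, after a delay, a test food recovery effect, each through a spawned effect executor actor.
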(event Custom|InitCharacterData
  ;[0.05048 0.1133 0.15 0.5] Bind Events for character attribute updates
  (bind _playerinventory (Class|BPIPlayerController|GetPlayerInventory(Message) (Components|GetOwner)))
  (EventDispatchers|AssignOnWeightChange _playerinventory (delegate Custom|OnWeightChange_Event))
  (bind _playerhotbar (Class|BPIPlayerController|GetPlayerHotbar(Message) (Components|GetOwner)))
  (EventDispatchers|BindEventtoOnWeightChange _playerhotbar (delegate Custom|OnWeightChange_Event)))

(event Custom|OnWeightChange_Event
  (params (TotalWeight :type Float%20%28double-precision%29))
  ;[0.05048 0.1133 0.15 0.5] Bind Events for character attribute updates
  (Inventory|UpdateInventoryTotalWeight))

(event EventBeginPlay
  (bind _abilitysystemcomp (Variables|Default|GetAbilitySystemComp))
  (bind _abilitysystemcomp_2 (Variables|Default|GetAbilitySystemComp))
  (bind _s_gameplayeffectcontext (Utilities|Struct|MakeS_GameplayEffectContext 0 _abilitysystemcomp_2 _abilitysystemcomp_2))
  (bind _s_gameplayeffectcontext_2 (Utilities|Struct|MakeS_GameplayEffectContext 0 _abilitysystemcomp _abilitysystemcomp))
  (Networking|SwitchHasAuthority
    (:Authority
      (bind _returnvalue (Game|ConstructObjectfromClass "/Game/Core/Blueprints/Systems/AbilitySystem/GameplayEffects/GE_Weight_Bonus_Test.GE_Weight_Bonus_Test_C" _s_gameplayeffectcontext_2))
      (bind _returnvalue_2 (Game|SpawnActorfromClass "/Game/Core/Blueprints/Systems/AbilitySystem/BP_GameplayEffectExecutor.BP_GameplayEffectExecutor_C" (Math|Transform|MakeTransform "0, 0, 0" "0, 0, 0" "1.000000,1.000000,1.000000") "AlwaysSpawn" "MultiplyWithRoot" self _returnvalue _s_gameplayeffectcontext_2 0))
      (Default|ApplyEffect _returnvalue_2)
      (Utilities|FlowControl|Delay 2e+01)
      (bind _returnvalue_3 (Game|ConstructObjectfromClass "/Game/Core/Blueprints/Systems/AbilitySystem/GameplayEffects/GE_Food_Recovery_Test.GE_Food_Recovery_Test_C" _s_gameplayeffectcontext))
      (bind _returnvalue_4 (Game|SpawnActorfromClass "/Game/Core/Blueprints/Systems/AbilitySystem/BP_GameplayEffectExecutor.BP_GameplayEffectExecutor_C" (Math|Transform|MakeTransform "0, 0, 0" "0, 0, 0" "1.000000,1.000000,1.000000") "AlwaysSpawn" "MultiplyWithRoot" self _returnvalue_3 _s_gameplayeffectcontext 0))
      (Default|ApplyEffect _returnvalue_4))))

(fn ConstructionScript)

(fn UpdateInventoryTotalWeight
  (bind _playerinventory (Class|BPIPlayerController|GetPlayerInventory(Message) (Components|GetOwner)))
  (bind _playerhotbar (Class|BPIPlayerController|GetPlayerHotbar(Message) (Components|GetOwner)))
  (Default|SetAttributeInstant (Variables|Default|GetCharacterAttributeComp) "(TagName=\"Attribute.Base.Weight\")" "NewEnumerator3" (+ (Variables|/Game/Core/Blueprints/Systems/InventorySystem/PrimaryComponent/BPC_Inventory.BPC_Inventory_C|GetTotalWeight _playerhotbar) (Variables|/Game/Core/Blueprints/Systems/InventorySystem/PrimaryComponent/BPC_Inventory.BPC_Inventory_C|GetTotalWeight _playerinventory))))

(fn GetCharacterAttributeComp
  (return (Variables|Default|GetCharacterAttributeComp)))

(fn GetAbilitySystemComp
  (return (Variables|Default|GetAbilitySystemComp)))

(fn GetAttributeSystemComp
  (return (Variables|Default|GetCharacterAttributeComp)))

(fn GetGameplayTagsComp
  (return (Variables|Default|GetGameplayTagsComp)))

(fn GetMyPlayerState
  (return self))

(fn HasGameplayTag
  (params (Tag :type Gameplay%20Tag%20Structure))
  (bind _result (Default|HasActiveTag (Variables|Default|GetGameplayTagsComp) Tag))
  (return _result))

(fn SetGameplayTag
  (params (Tag :type Gameplay%20Tag%20Structure) (Active :type Boolean))
  (Default|SetGameplayTag (Variables|Default|GetGameplayTagsComp) Tag Active))