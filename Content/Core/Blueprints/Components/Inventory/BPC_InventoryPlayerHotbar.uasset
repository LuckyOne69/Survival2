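; Player hotbar inventory component that maps ten Enhanced Input hotbar keys to slot selection.
; Selection broadcasts OnHotbarSlotSelected with the slot's item state, then requests equipping through TryToEquipItem_SERVER.
; Reselecting the equipped slot unequips it and broadcasts again, keeping non-equippable items highlighted.
; Equip and unequip are placeholders that only update the equipped index and print TODO messages.
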(event Custom|SetSelectedSlotIndex
  (params (SelectedSlotIndex :type Integer))
  (bind _output_get (Variables|Default|SetSelectSlotIndex SelectedSlotIndex))
  (bind _hasitem (CallFunction|TryGetSlotItemDataAsset _output_get))
  (Default|CallOnHotbarSlotSelected _hasitem _output_get)
  (if (== (Variables|Default|GetEquippedHotbarSlotIndex) (Variables|Default|GetSelectSlotIndex))
    (CallFunction|UnequipCurrentItem)
    ;[0.15 0.15 0.15 0.5] Not Equippable items, highlighted all time
    (bind _itemdataasset (CallFunction|TryGetSlotItemDataAsset (Variables|Default|GetSelectSlotIndex)))
    (bind _itemdataasset_2 (CallFunction|ResolveSoftItemDataReference _itemdataasset))
    (bind _returnvalue (Class|BPIItemData|IsItemEquippable(Message) _itemdataasset_2))
    (Default|CallOnHotbarSlotSelected (not _returnvalue) (Variables|Default|GetSelectSlotIndex))
    (else
      (CallFunction|TrytoEquipItemSERVER (Variables|Default|GetSelectSlotIndex)))))

(event Custom|UnequipCurrentItem
  ;[0.15 0.15 0.15 0.5] Equip / UnEquip item
  (bind _output_get (Variables|Default|SetEquippedHotbarSlotIndex -1))
  (CallFunction|PrintTodo "Unequip Slot Index" (Utilities|String|ToString(Integer) _output_get) true))

(event Custom|TryToEquipItem_SERVER
  (params (SlotIndex :type Integer))
  ;[0.15 0.15 0.15 0.5] Equip / UnEquip item
  (bind _output_get (Variables|Default|SetEquippedHotbarSlotIndex SlotIndex))
  (bind _itemdataasset (CallFunction|TryGetSlotItemDataAsset _output_get))
  (CallFunction|PrintTodo "Try to equipp item Slot" (Utilities|String|Append (Utilities|String|ToString(Integer) _output_get) "Asset: " (Utilities|ToString(SoftObjectReference) _itemdataasset)) true))

(event Input|EnhancedActionEvents|EnhancedInputActionIA_Hotbar_01
  (params (ActionValue :type Boolean) (ElapsedSeconds :type Float%20%28double-precision%29) (TriggeredSeconds :type Float%20%28double-precision%29) (InputAction :type Input%20Action%20Object%20Reference :default "/Game/Core/Data/Input/Actions/Hotbar/IA_Hotbar_01.IA_Hotbar_01"))
  ;[0.15 0.15 0.15 0.5] Hotbar keys
  (CallFunction|SetSelectedSlotIndex))

(event Input|EnhancedActionEvents|EnhancedInputActionIA_Hotbar_00
  (params (ActionValue :type Boolean) (ElapsedSeconds :type Float%20%28double-precision%29) (TriggeredSeconds :type Float%20%28double-precision%29) (InputAction :type Input%20Action%20Object%20Reference :default "/Game/Core/Data/Input/Actions/Hotbar/IA_Hotbar_00.IA_Hotbar_00"))
  ;[0.15 0.15 0.15 0.5] Hotbar keys
  (CallFunction|SetSelectedSlotIndex 9))

(event Input|EnhancedActionEvents|EnhancedInputActionIA_Hotbar_02
  (params (ActionValue :type Boolean) (ElapsedSeconds :type Float%20%28double-precision%29) (TriggeredSeconds :type Float%20%28double-precision%29) (InputAction :type Input%20Action%20Object%20Reference :default "/Game/Core/Data/Input/Actions/Hotbar/IA_Hotbar_02.IA_Hotbar_02"))
  ;[0.15 0.15 0.15 0.5] Hotbar keys
  (CallFunction|SetSelectedSlotIndex 1))

(event Input|EnhancedActionEvents|EnhancedInputActionIA_Hotbar_03
  (params (ActionValue :type Boolean) (ElapsedSeconds :type Float%20%28double-precision%29) (TriggeredSeconds :type Float%20%28double-precision%29) (InputAction :type Input%20Action%20Object%20Reference :default "/Game/Core/Data/Input/Actions/Hotbar/IA_Hotbar_03.IA_Hotbar_03"))
  ;[0.15 0.15 0.15 0.5] Hotbar keys
  (CallFunction|SetSelectedSlotIndex 2))

(event Input|EnhancedActionEvents|EnhancedInputActionIA_Hotbar_04
  (params (ActionValue :type Boolean) (ElapsedSeconds :type Float%20%28double-precision%29) (TriggeredSeconds :type Float%20%28double-precision%29) (InputAction :type Input%20Action%20Object%20Reference :default "/Game/Core/Data/Input/Actions/Hotbar/IA_Hotbar_04.IA_Hotbar_04"))
  ;[0.15 0.15 0.15 0.5] Hotbar keys
  (CallFunction|SetSelectedSlotIndex 3))

(event Input|EnhancedActionEvents|EnhancedInputActionIA_Hotbar_05
  (params (ActionValue :type Boolean) (ElapsedSeconds :type Float%20%28double-precision%29) (TriggeredSeconds :type Float%20%28double-precision%29) (InputAction :type Input%20Action%20Object%20Reference :default "/Game/Core/Data/Input/Actions/Hotbar/IA_Hotbar_05.IA_Hotbar_05"))
  ;[0.15 0.15 0.15 0.5] Hotbar keys
  (CallFunction|SetSelectedSlotIndex 4))

(event Input|EnhancedActionEvents|EnhancedInputActionIA_Hotbar_06
  (params (ActionValue :type Boolean) (ElapsedSeconds :type Float%20%28double-precision%29) (TriggeredSeconds :type Float%20%28double-precision%29) (InputAction :type Input%20Action%20Object%20Reference :default "/Game/Core/Data/Input/Actions/Hotbar/IA_Hotbar_06.IA_Hotbar_06"))
  ;[0.15 0.15 0.15 0.5] Hotbar keys
  (CallFunction|SetSelectedSlotIndex 5))

(event Input|EnhancedActionEvents|EnhancedInputActionIA_Hotbar_07
  (params (ActionValue :type Boolean) (ElapsedSeconds :type Float%20%28double-precision%29) (TriggeredSeconds :type Float%20%28double-precision%29) (InputAction :type Input%20Action%20Object%20Reference :default "/Game/Core/Data/Input/Actions/Hotbar/IA_Hotbar_07.IA_Hotbar_07"))
  ;[0.15 0.15 0.15 0.5] Hotbar keys
  (CallFunction|SetSelectedSlotIndex 6))

(event Input|EnhancedActionEvents|EnhancedInputActionIA_Hotbar_08
  (params (ActionValue :type Boolean) (ElapsedSeconds :type Float%20%28double-precision%29) (TriggeredSeconds :type Float%20%28double-precision%29) (InputAction :type Input%20Action%20Object%20Reference :default "/Game/Core/Data/Input/Actions/Hotbar/IA_Hotbar_08.IA_Hotbar_08"))
  ;[0.15 0.15 0.15 0.5] Hotbar keys
  (CallFunction|SetSelectedSlotIndex 7))

(event Input|EnhancedActionEvents|EnhancedInputActionIA_Hotbar_09
  (params (ActionValue :type Boolean) (ElapsedSeconds :type Float%20%28double-precision%29) (TriggeredSeconds :type Float%20%28double-precision%29) (InputAction :type Input%20Action%20Object%20Reference :default "/Game/Core/Data/Input/Actions/Hotbar/IA_Hotbar_09.IA_Hotbar_09"))
  ;[0.15 0.15 0.15 0.5] Hotbar keys
  (CallFunction|SetSelectedSlotIndex 8))

(event EventBeginPlay
  ;[0.15 0.15 0.15 0.5] Begin play
  (|CallParentFunction)
  (bind _playercharacter (Class|BPICharacter|GetPlayerCharacterRef(Message) (Components|GetOwner)))
  (Variables|References|SetPlayerCharacter _playercharacter))

(event EventEndPlay
  (params (EndPlayReason :type EEndPlayReason%20Enum :default "Destroyed"))
  ;[0.15 0.15 0.15 0.5] Begin play
  (EventDispatchers|UnbindallEventsfromOnHotbarSlotSelected))

(fn TryGetSlotItemDataAsset
  (params (Index :type Integer))
  (bind (_isvalid _slot) (CallFunction|GetSlotatIndex Index))
  (if (and _isvalid (CallFunction|IsSlotEmpty _slot))
    (return false 0)
    (else
      (return true (Utilities|Struct|BreakS_InventorySlot _slot)))))