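; Item component that turns gameplay tag triggers from an equipped item into server-applied use or consume effects.
; On equip, it binds the item's impact trigger tags on the owning character.
; Triggers run a client camera sphere trace, which the server re-traces and checks for range, actor, position and normal.
; Valid hits and trace-free Consume Impact triggers apply Gameplay Effects to the owning character, not the hit actor.
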(event Custom|OnItemEquipped_Event
  ;[0.15 0.15 0.15 0.5] When the item is equipped, all gameplay tag listeners locally for impact handling are registered so the item can react to hit events correctly.
  (CallFunction|BindImpactListenerCLIENT))

(event Custom|BindImpactListener_CLIENT
  ;[0.15 0.15 0.15 0.5] When the item is equipped, all gameplay tag listeners locally for impact handling are registered so the item can react to hit events correctly.
  (bind _itemdatacomp (Class|BPIItemMaster|GetItemDataComp(Message) (Components|GetOwner)))
  (bind _itemdata (Class|BPIItemData|GetItemData(Message) _itemdatacomp))
  (Utilities|IsValid _itemdata
    (:Is%20Valid
      (CallFunction|OnItemDataResolvedEvent))
    (:Is%20Not%20Valid
      (EventDispatchers|AssignOnItemDataResolved _itemdatacomp (delegate Custom|OnItemDataResolved_Event)))))

(event Custom|ValidateAndApplylmpactTraceReport_SERVER
  (params (InTraceReport :type S%20Trace%20Hit%20Client%20Report%20Structure))
  ;[0.15 0.15 0.15 0.5] Receives the TraceReport from the client, validates it on the server using ValidatelmpactTraceReportOnServer
  ; and applies the hit via ApplyValidatedImpact if the report is valid.
  (bind (_ishitvalid _outhit) (CallFunction|ValidateImpactTraceReportonServer InTraceReport))
  (if _ishitvalid
    (CallFunction|ApplyValidatedImpact _outhit)
    (else
      (CallFunction|PrintError "Server tryce validation failed" "" true))))

(event Custom|ExecuteConsumeImpact_SERVER
  ;[0.15 0.15 0.15 0.5] Handles the special Consume Impact case by retrieving the item's consumable data and applying its defined Gameplay Effect directly to the
  ; character.
  (bind _itemdatacomp (Class|BPIItemMaster|GetItemDataComp(Message) (Components|GetOwner)))
  (bind (_isconsumible _itemconsumibleinfo) (Class|BPIItemData|GetConsumibleInfo(Message) _itemdatacomp))
  (if _isconsumible
    (CallFunction|ApplyItemUseEffect (.gameplayeffectclass _itemconsumibleinfo))))

(event Custom|ApplyItemUseEffect
  (params (GameplayEffectClass :type Gameplay%20Effect%20Base%20Soft%20Class%20Reference))
  ;[0.15 0.15 0.15 0.5] Applies the Gameplay Effect to the character through the Ability System.
  (bind _returnvalue (Utilities|IsValidSoftClassReference GameplayEffectClass))
  (if _returnvalue
    (bind _playercharacter (Class|BPIItemEquippable|GetOwningPlayerCharacter(Message) (Components|GetOwner)))
    (bind _abilitysystemcomp (Class|BPIAbilitySystemProvider|GetAbilitySystemComp(Message) _playercharacter))
    (Default|ApplyGameplyEffecttoSelf _abilitysystemcomp GameplayEffectClass)))

(event Custom|OnItemDataResolved_Event
  ;[0.15 0.15 0.15 0.5] When the item is equipped, all gameplay tag listeners locally for impact handling are registered so the item can react to hit events correctly.
  (bind _itemequippableinfo (Class|BPIItemData|GetEquippableInfo(Message) (stale Custom|BindImpactListener_CLIENT _itemdatacomp)))
  (bind _returnvalue (CallFunction|IsTagContainerNotEmpty (Utilities|Struct|BreakS_ItemEquippableRow _itemequippableinfo)))
  (if _returnvalue
    (bind _playercharacter (Class|BPIItemEquippable|GetOwningPlayerCharacter(Message) (Components|GetOwner)))
    (bind _gameplaytagscomp (Class|BPIAbilitySystemProvider|GetGameplayTagsComp(Message) _playercharacter))
    (Default|BindTagListener _gameplaytagscomp self (Utilities|Struct|BreakS_ItemEquippableRow _itemequippableinfo))))

(event EventBeginPlay
  ;[0.15 0.15 0.15 0.5] When the item is equipped, all gameplay tag listeners locally for impact handling are registered so the item can react to hit events correctly.
  (bind _itemequippablecomp (Class|BPIItemEquippable|GetItemEquippableComponent(Message) (Components|GetOwner)))
  (EventDispatchers|AssignOnItemEquipped _itemequippablecomp (delegate Custom|OnItemEquipped_Event)))

(event EventEndPlay
  (params (EndPlayReason :type EEndPlayReason%20Enum :default "Destroyed"))
  ;[0.15 0.15 0.15 0.5] Remove all impact listeners
  (bind _playercharacter (Class|BPIItemEquippable|GetOwningPlayerCharacter(Message) (Components|GetOwner)))
  (bind _gameplaytagscomp (Class|BPIAbilitySystemProvider|GetGameplayTagsComp(Message) _playercharacter))
  (Utilities|IsValid _gameplaytagscomp
    (:Is%20Valid
      (Default|UnbindListenerfromAllTags _gameplaytagscomp self))))

(event EventOnTagChanged
  (params (Context :type S%20Gameplay%20Tag%20Changed%20Context%20Structure))
  ;[0.15 0.15 0.15 0.5] Reacts to impact events. Normal impacts trigger a client trace and send the result to the server via ValidateAndApplyImpactTrace_SERVER,
  ; while the special Consume Impact tag is handled separately through ExecuteConsumelmpact_SERVER.
  (if (.isactive Context)
    (|SwitchGameplayTag (.tag Context)
      (:Default
        (bind (_hashit _tracereport) (CallFunction|TraceTargetonClient))
        (if _hashit
          (CallFunction|ValidateandApplylmpactTraceReportSERVER _tracereport)))
      (:Ability.Trigger.ConsumeImpact
        (CallFunction|ExecuteConsumeImpactSERVER)))))

(fn TraceTargetonClient
  ;[0.15 0.15 0.15 0.5] Performs a forward sphere trace from the player's camera to detect impact targets within the equipped item's range.
  ; The result is converted into a compact hit report for replication and further server-side impact handling.
  (bind _itemdatacomp (Class|BPIItemMaster|GetItemDataComp(Message) (Components|GetOwner)))
  (bind (_isequippable _itemequippableinfo) (Class|BPIItemData|GetEquippableInfo(Message) _itemdatacomp))
  (if _isequippable
    (bind _playercharacter (Class|BPIItemEquippable|GetOwningPlayerCharacter(Message) (Components|GetOwner)))
    (bind (_location _rotation) (Class|BPICharacter|GetTraceCameraData(Message) _playercharacter))
    (bind (_outhit _returnvalue) (Collision|SphereTraceByChannel _location (+ _location (* (Math|Vector|GetForwardVector _rotation) (Utilities|Struct|BreakS_ItemEquippableRow _itemequippableinfo))) 5.0 "TraceTypeQuery1" false (Utilities|Array|MakeArray _playercharacter) "ForDuration"))
    (return _returnvalue (CallFunction|MakeTraceClientHitReport (Transformation|GetActorLocation _playercharacter) _outhit))
    (else
      (return false ""))))

(fn ValidateImpactTraceReportonServer
  (params (TraceReport :type S%20Trace%20Hit%20Client%20Report%20Structure))
  (bind (_tracestart _traceend) (Utilities|Struct|BreakS_TraceHitClientReport TraceReport))
  (bind (_actorlocation _tracestart_2 _traceend_2 _hitlocation) (Utilities|Struct|BreakS_TraceHitClientReport TraceReport))
  (bind (_hitactor _hitlocation_2 _hitnormal) (Utilities|Struct|BreakS_TraceHitClientReport TraceReport))
  ;[0.15 0.15 0.15 0.5] The server validates the client's trace report by checking if the reported hit location is within the allowed use distance of the equipped item.
  ; We compare the player position to the impact location and add a small tolerance factor by multiplying the maximum distance with 1.1.
  (bind _itemdatacomp (Class|BPIItemMaster|GetItemDataComp(Message) (Components|GetOwner)))
  (bind (_isequippable _itemequippableinfo) (Class|BPIItemData|GetEquippableInfo(Message) _itemdatacomp))
  (if _isequippable
    (bind _playercharacter (Class|BPIItemEquippable|GetOwningPlayerCharacter(Message) (Components|GetOwner)))
    (if (and (< (Math|Vector|Distance(Vector) (Transformation|GetActorLocation _playercharacter) _actorlocation) 1e+01) (Math|Float|InRange(Float) (Math|Vector|Distance(Vector) _tracestart_2 _hitlocation) 0.0 (* (Utilities|Struct|BreakS_ItemEquippableRow _itemequippableinfo) 1.1)))
      (bind (_outhits _returnvalue) (Collision|MultiSphereTraceByChannel _tracestart _traceend 5.0 "TraceTypeQuery1" false (Utilities|Array|MakeArray _playercharacter) "None"))
      ;[0.15 0.15 0.15 0.5] Here we validate the reported hit by comparing the client trace data with the server trace. We check that both hit the same actor, that the impact location is close enough within a small distance
      ; tolerance, and that the hit normal points in the same direction within about eighteen degrees using a Dot Product check greater than 0.95.
      ; Only when all these conditions are true the hit is accepted as valid and passed on, otherwise it is rejected.
      (if _returnvalue
        (for _array_element _outhits
          (if (Math|Boolean|ANDBoolean (< (Math|Vector|Distance(Vector) (.ImpactPoint (Collision|BreakHitResult _array_element)) _hitlocation_2) 15.0) (> (Math|Vector|DotProduct _hitnormal (.ImpactNormal (Collision|BreakHitResult _array_element))) 0.95) (== _hitactor (.HitActor (Collision|BreakHitResult _array_element))))
            (return true _array_element))))
      (return false "")
      (else
        (return false "")))
    (else
      (return false ""))))

(fn ApplyValidatedImpact
  (params (HitResult :type Hit%20Result%20Structure))
  (bind _itemdatacomp (Class|BPIItemMaster|GetItemDataComp(Message) (Components|GetOwner)))
  (LocalVariables|SetItemDataComp _itemdatacomp)
  (Utilities|FlowControl|Sequence
    (:then_0
      ;[0.15 0.15 0.15 0.5] Applr item use effect y impact etc.
      (CallFunction|ApplyItemUseEffect (.AppliedUseEffectClass (Default|GetAppliedUseEffectClass (LocalVariables|GetItemDataComp)))))))