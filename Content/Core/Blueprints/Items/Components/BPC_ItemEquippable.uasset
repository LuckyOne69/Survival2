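; Item component that handles equipping and unequipping its owning item on the player character.
; On equip, it reads equippable data through interface messages, sets the character's stance and, for right-hand or both-hands slots, snaps the item to a hand socket on the character mesh.
; Unequipping resets the stance without detaching the item.
; Event dispatchers announce equip and unequip, and their bindings are cleared on EndPlay.
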(event Custom|SetEquippableStance
  (params (EquipmentStance :type E_ItemEquipmentType%20Enum :default "NewEnumerator0"))
  ;[0.15 0.15 0.15 0.5] Getter / Setter
  (bind _playercharacter (Class|BPIItemEquippable|GetOwningPlayerCharacter(Message) (Components|GetOwner)))
  (Default|SetEquippedStance _playercharacter EquipmentStance))

(event Custom|UnequippedItem
  ;[0.15 0.15 0.15 0.5] Equip / Unequip Items
  (CallFunction|SetEquippableStance "NewEnumerator0")
  (Default|CallOnItemUnEquipped))

(event Custom|EquipItem
  (bind _returnvalue (Components|GetOwner))
  ;[0.15 0.15 0.15 0.5] Equip / Unequip Items
  (bind _itemdatacomp (Class|BPIItemMaster|GetItemDataComp(Message) (Components|GetOwner)))
  (bind (_isvalid _itemequippabledata) (Default|GetEquippableData _itemdatacomp))
  (if _isvalid
    (CallFunction|SetEquippableStance (Variables|/Game/Core/Blueprints/PrimaryDataAssets/Items/PDA_ItemEquippableMaster.PDA_ItemEquippableMaster_C|GetEquipmentType _itemequippabledata))
    (switch Utilities|FlowControl|Switch|SwitchonE_ItemEquipmentSlot (Variables|/Game/Core/Blueprints/PrimaryDataAssets/Items/PDA_ItemEquippableMaster.PDA_ItemEquippableMaster_C|GetEquipmentSlot _itemequippabledata)
      (:NewEnumerator1
        _)
      (:NewEnumerator2
        _))
    (bind _playercharacter (Class|BPIItemEquippable|GetOwningPlayerCharacter(Message) _returnvalue))
    (bind _skeletalmeshcomp (Class|BPICharacter|GetPlayerCharacterMesh(Message) _playercharacter))
    (Transformation|AttachComponentToComponent _returnvalue _skeletalmeshcomp (Utilities|Select :Index (Variables|/Game/Core/Blueprints/PrimaryDataAssets/Items/PDA_ItemEquippableMaster.PDA_ItemEquippableMaster_C|GetAttachSocket _itemequippabledata) :NewEnumerator0 "EquipRightHandSocket" :NewEnumerator1 "EquipLeftHandSocket") "SnapToTarget" "SnapToTarget" "SnapToTarget" true)
    (Default|CallOnItemEquipped)))

(event EventEndPlay
  (params (EndPlayReason :type EEndPlayReason%20Enum :default "Destroyed"))
  ;[0.15 0.15 0.15 0.5] Begin / End Play
  (EventDispatchers|UnbindallEventsfromOnItemEquipped)
  (EventDispatchers|UnbindallEventsfromOnItemUnEquipped))