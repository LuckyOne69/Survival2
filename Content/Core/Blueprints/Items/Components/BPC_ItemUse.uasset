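; Item component that handles use of an equippable item in single, automatic or burst mode.
; On equip it reads mode, rate, burst count and primary ability from the item data.
; Server start/stop triggers fire an immediate use, then a looping timer repeats it; bursts ignore stop, and restarting cancels a pending stop.
; On authority, each use activates the primary Gameplay Ability on the owning character's ability system.
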(event Custom|OnItemEquipped_Event
  ;[0.15 0.15 0.15 0.5] Initialize Use Data
  (bind _itemdatacomp (Class|BPIItemMaster|GetItemDataComp(Message) (Components|GetOwner)))
  (bind _itemequippableinfo (Class|BPIItemData|GetEquippableInfo(Message) _itemdatacomp))
  (Variables|Default|SetUseInterval (/ 1.0 (.UseInterval (Utilities|Struct|BreakS_ItemEquippableRow _itemequippableinfo))))
  (Variables|Default|SetCurrentUsageMode (.UseMode (Utilities|Struct|BreakS_ItemEquippableRow _itemequippableinfo)))
  (Variables|Default|SetUseBurstCount (.UseBustCount (Utilities|Struct|BreakS_ItemEquippableRow _itemequippableinfo)))
  (Variables|Default|SetPrimaryUseAbility (.Value (Utilities|Map|Find (.ItemUseAbilityMap (Utilities|Struct|BreakS_ItemEquippableRow _itemequippableinfo)) "(TagName=\"Ability.ItemUse.Primary\")"))))

(event Custom|TriggerStartUse_SERVER
  ;[0.15 0.15 0.15 0.5] Trigger Start/Stop Use
  (if (and (Variables|Default|GetShouldStopUsing) (Variables|Default|GetIsUsing))
    (Variables|Default|SetShouldStopUsing false)
    (elif (and (Variables|Default|GetIsUsable) (not (Variables|Default|GetIsUsing)))
      (Variables|Default|SetShouldStopUsing false)
      (Variables|Default|SetIsUsing true)
      (Default|CallOnItemUsed)
      (switch Utilities|FlowControl|Switch|SwitchonE_ItemUseMode (Variables|Default|GetCurrentUsageMode)
        (:NewEnumerator0
          (CallFunction|StartUsingLoopTimer 1))
        (:NewEnumerator1
          (CallFunction|StartUsingLoopTimer 999))
        (:NewEnumerator2
          (CallFunction|StartUsingLoopTimer (Variables|Default|GetUseBurstCount)))))))

(event Custom|TriggerStopUse_SERVER
  ;[0.15 0.15 0.15 0.5] Trigger Start/Stop Use
  (if (Utilities|Enum|NotEqual(Enum) (Variables|Default|GetCurrentUsageMode) "NewEnumerator2")
    (Variables|Default|SetShouldStopUsing true)))

(event Custom|OnItemUsed_Event
  ;[0.15 0.15 0.15 0.5] Execute Use Ability on item usage
  (bind _primaryuseability (Variables|Default|GetPrimaryUseAbility)
    (:then
      (bind _playercharacter (Class|BPIItemEquippable|GetOwningPlayerCharacter(Message) (Components|GetOwner)))
      (bind _abilitysystemcomp (Class|BPIAbilitySystemProvider|GetAbilitySystemComp(Message) _playercharacter))
      (Default|TryActivateAbilitybyClass _abilitysystemcomp _primaryuseability))
    (:else
      (CallFunction|PrintError "Primary use ability is invalid" "" true))))

(event Custom|StartUsingLoopTimer
  (params (UsingLoopAmount :type Integer))
  ;[0.15 0.15 0.15 0.5] Timer For Burst/Automatic Mode
  (Variables|Default|SetUsingCounter UsingLoopAmount)
  (bind _returnvalue (Utilities|Time|SetTimerbyEvent (delegate Custom|HandelItemUsing_Event) (Variables|Default|GetUseInterval) true))
  (Variables|Default|SetUseIntervalTimerRef _returnvalue))

(event Custom|HandelItemUsing_Event
  ;[0.15 0.15 0.15 0.5] Timer For Burst/Automatic Mode
  (bind _result (Math|Integer|DecrementInt (Variables|Default|GetUsingCounter))
    (:%20%20
      (if (Math|Boolean|ANDBoolean (> _result 0) (Variables|Default|GetIsUsing) (not (Variables|Default|GetShouldStopUsing)))
        (Default|CallOnItemUsed)
        (else
          (CallFunction|ReadytoUseAgain))))))

(event Custom|ReadyToUseAgain
  ;[0.15 0.15 0.15 0.5] Trigger Start/Stop Use
  (Default|CallOnItemUsedStop)
  (Variables|Default|SetIsUsing false)
  (Utilities|Time|ClearandInvalidateTimerbyHandle (Variables|Default|GetUseIntervalTimerRef)))

(event EventBeginPlay
  ;[0.15 0.15 0.15 0.5] Initialize Use Data
  (bind _itemequippablecomp (Class|BPIItemEquippable|GetItemEquippableComponent(Message) (Components|GetOwner)))
  (EventDispatchers|AssignOnItemEquipped _itemequippablecomp (delegate Custom|OnItemEquipped_Event))
  (Networking|SwitchHasAuthority
    (:Authority
      ;[0.15 0.15 0.15 0.5] Execute Use Ability on item usage
      (EventDispatchers|AssignOnItemUsed (delegate Custom|OnItemUsed_Event)))))

(event EventEndPlay
  (params (EndPlayReason :type EEndPlayReason%20Enum :default "Destroyed"))
  ;[0.15 0.15 0.15 0.5] Initialize Use Data
  (CallFunction|ReadytoUseAgain))