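; Item component that holds a soft reference to an item data asset and exposes its properties to the owning item.
; SetItemDataAsset stores the reference, resolves it into ItemData, and logs errors when it is invalid or fails to resolve.
; All other getters and type checks, such as ammo, armor, consumable, durability, stacking and fuel, forward straight to ItemData without validity checks.
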(fn SetItemDataAsset
  (params (ItemDataAsset :type PDA%20Item%20Data%20Soft%20Object%20Reference))
  (Variables|Default|SetItemDataAsset ItemDataAsset)
  (if (Utilities|IsValidSoftObjectReference ItemDataAsset)
    (bind _itemdata (CallFunction|ResolveSoftItemDataReference (Variables|Default|GetItemDataAsset)))
    (bind _output_get (Variables|Default|SetItemData _itemdata))
    (Utilities|IsValid _output_get
      (:Is%20Not%20Valid
        _))
    (else
      (CallFunction|PrintError "ItemDataAsset is not valid in" (Utilities|GetDisplayName self) true)))
  (CallFunction|PrintError "ItemDataAsset Reference failed to Resolve in BP_ItemMaster" (Utilities|ToString(SoftObjectReference) (Variables|Default|GetItemDataAsset)) true))

(fn GetItemDataAsset
  (return (Variables|Default|GetItemDataAsset)))

(fn GetAmmoInfo
  (bind (_useammo _itemammoprofileinfo) (Default|GetAmmoInfo (Variables|Default|GetItemData)))
  (return _useammo _itemammoprofileinfo))

(fn GetArmorInfo
  (bind (_isarmor _itemarmorprofileinfo) (Default|GetArmorInfo (Variables|Default|GetItemData)))
  (return _isarmor _itemarmorprofileinfo))

(fn GetConsumibleInfo
  (bind (_isconsumible _itemconsumibleinfo) (Default|GetConsumibleInfo (Variables|Default|GetItemData)))
  (return _isconsumible _itemconsumibleinfo))

(fn GetDurabilityInfo
  (bind (_usesdurability _itemdurabilityinfo) (Default|GetDurabilityInfo (Variables|Default|GetItemData)))
  (return _usesdurability _itemdurabilityinfo))

(fn GetEquippableInfo
  (bind (_isequippable _itemequippableinfo) (Default|GetEquippableInfo (Variables|Default|GetItemData)))
  (return _isequippable _itemequippableinfo))

(fn GetHarvestToolInfo
  (bind _itemharvesttoolinfo (Default|GetHarvestToolInfo (Variables|Default|GetItemData)))
  (return _itemharvesttoolinfo))

(fn GetItemData
  (bind _itemdata (Default|GetItemData (Variables|Default|GetItemData)))
  (return _itemdata))

(fn GetItemIcon
  (bind _icon (Default|GetItemIcon (Variables|Default|GetItemData)))
  (return _icon))

(fn GetStackableInfo
  (bind (_isstackable _stacksize) (Default|GetStackableInfo (Variables|Default|GetItemData)))
  (return _isstackable _stacksize))

(fn HasDurability
  (bind _returnvalue (Default|HasDurability (Variables|Default|GetItemData)))
  (return _returnvalue))

(fn IsAmmo
  (bind _returnvalue (Default|IsAmmo (Variables|Default|GetItemData)))
  (return _returnvalue))

(fn IsArmor
  (bind _returnvalue (Default|IsArmor (Variables|Default|GetItemData)))
  (return _returnvalue))

(fn IsConsumable
  (bind _returnvalue (Default|IsConsumable (Variables|Default|GetItemData)))
  (return _returnvalue))

(fn IsEquippable
  (bind _returnvalue (Default|IsEquippable (Variables|Default|GetItemData)))
  (return _returnvalue))

(fn IsFuel
  (bind _returnvalue (Default|IsFuel (Variables|Default|GetItemData)))
  (return _returnvalue))

(fn IsHarvestTool
  (bind _returnvalue (Default|IsHarvestTool (Variables|Default|GetItemData)))
  (return _returnvalue))

(fn IsResource
  (bind _returnvalue (Default|IsResource (Variables|Default|GetItemData)))
  (return _returnvalue))

(fn IsStackable
  (bind _returnvalue (Default|IsStackable (Variables|Default|GetItemData)))
  (return _returnvalue))