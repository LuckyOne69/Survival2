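; Melee weapon item component that plays attack animations on the owning character when the weapon is used.
; The use event runs a multicast that signals successful use, then reads the item's equipment type through message calls on the owner.
; It picks an axe montage for Melee or a spear montage for Spear, in first- or third-person form based on the active camera.
; The montage selection is hardcoded and marked as test code.
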(event Custom|ItemUsed_Multicast
  (bind _returnvalue (Components|GetOwner))
  (Default|CallOnWeaponUseSuccesfully)
  ;[0.15 0.006216 0.0092 0.5] Just For Test
  (bind _playercharacter (Class|BPIItemEquippable|GetOwningPlayerCharacter(Message) _returnvalue))
  (bind _itemdatacomp (Class|BPIItemMaster|GetItemDataComp(Message) _returnvalue))
  (bind _itemequippableinfo (Class|BPIItemData|GetEquippableInfo(Message) _itemdatacomp))
  (switch Utilities|FlowControl|Switch|SwitchonE_ItemEquipmentType (.EquipmentType (Utilities|Struct|BreakS_ItemEquippableRow _itemequippableinfo))
    (:NewEnumerator1
      (if (Variables|/Game/Core/Blueprints/Charactes/BP_PlayerCharacter.BP_PlayerCharacter_C|GetIsFirstPersonCameraActive _playercharacter)
        (Class|BPICharacter|CharPlayAnimMontage(Message) _playercharacter false "/Game/Core/Art/Characters/PlayerCharacter/Animations/Equipment/Melee/M_Axe_FP_Attack_Montage.M_Axe_FP_Attack_Montage")
        (else
          (Class|BPICharacter|CharPlayAnimMontage(Message) _playercharacter false "/Game/Core/Art/Characters/PlayerCharacter/Animations/Equipment/Melee/M_Axe_TP_Attack_Montage.M_Axe_TP_Attack_Montage"))))
    (:NewEnumerator6
      (if (Variables|/Game/Core/Blueprints/Charactes/BP_PlayerCharacter.BP_PlayerCharacter_C|GetIsFirstPersonCameraActive _playercharacter)
        (Class|BPICharacter|CharPlayAnimMontage(Message) _playercharacter false "/Game/Core/Art/Characters/PlayerCharacter/Animations/Equipment/Spear/M_Spear_FP_Attack_Montage.M_Spear_FP_Attack_Montage")
        (else
          (Class|BPICharacter|CharPlayAnimMontage(Message) _playercharacter false "/Game/Core/Art/Characters/PlayerCharacter/Animations/Equipment/Spear/M_Spear_TP_Attack_Montage.M_Spear_TP_Attack_Montage"))))))

(event EventHandleWeaponUsedEvent
  (CallFunction|ItemUsedMulticast))