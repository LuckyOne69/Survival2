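; Hand IK component for an equipped item that supplies left and right hand target transforms on the owning player character.
; MakeTransform reads a socket on the item's skeletal mesh in world space and converts it into a bone's space on the character mesh, with unit scale.
; The left target (LHIKSocket) is relative to hand_r and the right (RHIKSocket) to hand_l, each gated by its HasLHIK or HasRHIK flag.
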(event EventBeginPlay)

(event EventTick
  (params (DeltaSeconds :type Float%20%28single-precision%29)))

(fn MakeTransform
  (params (InSocketName :type Name) (BoneName :type Name))
  (bind _returnvalue (Components|GetOwner))
  (bind _skeletalmesh (Class|BPIItemEquippable|GetEquippedItemSkeletalMesh(Message) _returnvalue))
  (bind _playercharacter (Class|BPIItemEquippable|GetOwningPlayerCharacter(Message) _returnvalue))
  (bind _skeletalmeshcomp (Default|GetPlayerCharacterMesh _playercharacter))
  (return (Math|Transform|MakeTransform (.OutPosition (Class|SkinnedMeshComponent|TransformtoBoneSpace _skeletalmeshcomp BoneName (.location (Transformation|GetSocketTransform _skeletalmesh InSocketName "RTS_World")) (.rotation (Transformation|GetSocketTransform _skeletalmesh InSocketName "RTS_World")))) (.OutRotation (Class|SkinnedMeshComponent|TransformtoBoneSpace _skeletalmeshcomp BoneName (.location (Transformation|GetSocketTransform _skeletalmesh InSocketName "RTS_World")) (.rotation (Transformation|GetSocketTransform _skeletalmesh InSocketName "RTS_World")))) "1.000000,1.000000,1.000000")))

(fn GetLHIKTransform
  (if (Variables|HandIKComponent|GetHasLHIK)
    (return (CallFunction|MakeTransform "LHIKSocket" "hand_r"))))

(fn GetRHIKTransform
  (if (Variables|HandIKComponent|GetHasRHIK)
    (return (CallFunction|MakeTransform "RHIKSocket" "hand_l"))))