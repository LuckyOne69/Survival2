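; BP_ItemEquippableMaster is the base actor for equippable items, with placeholder start and stop use events that only print a to-do message.
; On BeginPlay, the authority tells its ItemEquippableComp to equip the item and binds OnDestroyed so that destroying the actor unequips it.
; Getter functions expose the item itself and resolve the owning player character through a message call on the actor's Owner.
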(event Custom|OnDestroyed_Event
  (params (DestroyedActor :type Actor%20Object%20Reference))
  ;[0.15 0.15 0.15 0.5] Initialization
  (Default|UnequippedItem (Variables|Default|GetItemEquippableComp)))

(event EventBeginPlay
  ;[0.15 0.15 0.15 0.5] Initialization
  (|CallParentFunction)
  (Networking|SwitchHasAuthority
    (:Authority
      (Game|AssignOnDestroyed (delegate Custom|OnDestroyed_Event))
      (Default|EquipItem (Variables|Default|GetItemEquippableComp)))))

(event EventStarUse
  ;[0.15 0.15 0.15 0.5] Trigger to use items
  (CallFunction|PrintTodo "Use Item" "" true))

(event EventStopUse
  ;[0.15 0.15 0.15 0.5] Trigger to use items
  (CallFunction|PrintTodo "Stop Use Item" "" true))

(fn ConstructionScript
  (|CallParentFunction))

(fn GetbyItemEquippable
  (return self))

(fn GetOwningPlayerCharacter
  (bind _playercharacter (Class|BPICharacter|GetBpPlayerCharacter(Message) (Components|GetOwner)))
  (return _playercharacter))