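; Actor component in the ability system that holds a replicated container of active gameplay tags and answers exact-match tag queries.
; Set events add or remove single or multiple tags, skipping redundant changes, then diff the container against its previous state.
; Each added or removed tag fires an any-tag-changed notification with a context struct.
; The ActiveTags OnRep runs the same diff against a cached copy, so clients raise notifications locally.
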(event Custom|SetGameplayTags
  (params (Tags :type Gameplay%20Tag%20Container%20Structure) (Enabled :type Boolean))
  ;[0.15 0.15 0.15 0.5] Set Gameplay Tag States
  (CallFunction|UpdateTagState Tags Enabled))

(event Custom|SetGameplayTag
  (params (Tag :type Gameplay%20Tag%20Structure) (Enabled :type Boolean))
  ;[0.15 0.15 0.15 0.5] Set Gameplay Tag States
  (CallFunction|UpdateTagState (GameplayTags|MakeGameplayTagContainerfromTag Tag) Enabled))

(fn UpdateTagState
  (params (Tags :type Gameplay%20Tag%20Container%20Structure) (Enabled :type Boolean))
  ;[0.15 0.15 0.15 0.5] Adds or removes the tags based on the Enabled value, prevents duplicates, and notifies via proccesstagdiffandnotify.
  (Variables|GameplayTagsComponent|SetPreActiveTags (Variables|GameplayTagsComponent|GetActiveTags))
  (for _array_element (GameplayTags|BreakGameplayTagContainer Tags)
    (if Enabled
      (if (not (GameplayTagsComponent|HasActiveTag _array_element))
        (GameplayTags|AddGameplayTag (Variables|GameplayTagsComponent|GetActiveTags) _array_element :!class /Script/GameplayTags.BlueprintGameplayTagLibrary))
      (elif (GameplayTagsComponent|HasActiveTag _array_element)
        (GameplayTags|RemoveGameplayTag (Variables|GameplayTagsComponent|GetActiveTags) _array_element :!class /Script/GameplayTags.BlueprintGameplayTagLibrary))))
  (CallFunction|ProcessTagDiffandNotify (Variables|GameplayTagsComponent|GetPreActiveTags) (Variables|GameplayTagsComponent|GetActiveTags)))

(fn HasActiveTag
  (params (tag :type Gameplay%20Tag%20Structure))
  ;[0.15 0.15 0.15 0.5] Checks if the provided tag exists in the list of currently active tags.                                   UUses exact match to ensure the tag must be present without partial hierarchy inclusion.
  (return (GameplayTags|HasTag (Variables|GameplayTagsComponent|GetActiveTags) tag true)))

(fn HasActiveTags
  (params (Tags :type Gameplay%20Tag%20Container%20Structure) (AllTags :type Boolean))
  ;[0.15 0.15 0.15 0.5] Returns true if the specified tag or any tag from the input container exists in the list of actrive tags.     Use the"All Tags" input to require all tags to be present instead of just one.
  (if AllTags
    (return (GameplayTags|HasAllTags (Variables|GameplayTagsComponent|GetActiveTags) Tags true))
    (else
      (return (GameplayTags|HasAnyTags (Variables|GameplayTagsComponent|GetActiveTags) Tags true)))))

(fn NotifyLocalTagChanges
  (params (TagChangeContext :type S%20Gameplay%20Tag%20Changed%20Context%20Structure))
  (Default|CallOnAnyTagChanged TagChangeContext))

(fn ProcessTagDiffandNotify
  (params (PrevContainer :type Gameplay%20Tag%20Container%20Structure) (NewContainer :type Gameplay%20Tag%20Container%20Structure))
  ;[0.15 0.15 0.15 0.5] Compares the Previous and current gameplay tag
  (Variables|GameplayTagsComponent|SetPreActiveTags NewContainer)
  (LocalVariables|SetTagChangeContext (Utilities|Struct|MakeS_GameplayTagChangedContext "(TagName=\"\")" NewContainer false))
  (for _array_element (GameplayTags|BreakGameplayTagContainer NewContainer)
    (bind _returnvalue (GameplayTags|RemoveGameplayTag PrevContainer _array_element :!class /Script/GameplayTags.BlueprintGameplayTagLibrary))
    (if (not _returnvalue)
      (bind _structout (Utilities|Struct|SetmembersinS_GameplayTagChangedContext (LocalVariables|GetTagChangeContext) _array_element true))
      (CallFunction|NotifyLocalTagChanges _structout)))
  (for _array_element_2 (GameplayTags|BreakGameplayTagContainer PrevContainer)
    (bind _structout_2 (Utilities|Struct|SetmembersinS_GameplayTagChangedContext (LocalVariables|GetTagChangeContext) _array_element_2 false))
    (CallFunction|NotifyLocalTagChanges _structout_2)))

(fn OnRepActiveTags
  ;[0.15 0.15 0.15 0.5] Called On Clients When The Replicated ActiveTags array is Updated.
  (CallFunction|ProcessTagDiffandNotify (Variables|GameplayTagsComponent|GetPreActiveTags) (Variables|GameplayTagsComponent|GetActiveTags)))