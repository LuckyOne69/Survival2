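; Gameplay attribute component that the server initializes from async-loaded base, threshold and derived-stat DataTables, then replicates to the client before signalling ready.
; Attributes are keyed by GameplayTag, with instant changes processed through a queue and persistent modifiers grouped by operator, removable by effect GUID.
; Each recalculated value is clamped, toggles threshold status tags on the owner, fires a change event and notifies the client.
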(event Custom|SetupAttributeFromDataTable
  (params (DT%20AttributeBaseValue :type Data%20Table%20Soft%20Object%20Reference) (DT%20AttributeThreshold :type Data%20Table%20Soft%20Object%20Reference) (DT%20AttributeDerivedStats :type Data%20Table%20Soft%20Object%20Reference))
  (Networking|SwitchHasAuthority
    (:Authority
      (CallFunction|InitializeBaseDefinitionData DT%20AttributeBaseValue)
      (CallFunction|InitializeThresholdData DT%20AttributeThreshold)
      (CallFunction|InitializeDerivedData DT%20AttributeDerivedStats))))

(event Custom|InitializeDerivedData
  (params (DT%20AttributeDerivedStats :type Data%20Table%20Soft%20Object%20Reference))
  (bind _output (Utilities|ResolveSoftReference DT%20AttributeDerivedStats))
  ;[0.15 0.15 0.15 0.5] Load Level scaled attribute
  (Utilities|AsyncLoadAsset DT%20AttributeDerivedStats
    (:Completed
      (bind _outrownames (DataTable|GetDataTableRowNames _output))
      (for _array_element _outrownames
        (bind _returnvalue (Utilities|GetDataTableRow _output _array_element)
          (:then
            (Utilities|Map|Add (Variables|AttributeSystemDerivedState|GetAttributeDerivedDefinitionMap) (Utilities|Struct|BreakS_AttributeInitRowDerivedStatValue _returnvalue) _returnvalue))))
      (AttributeSystemLoader|CheckIsAttributeSystemInitialize))))

(event Custom|ReplicateInitAttributeData_CLIENT
  (params (AttributeState :type Array%20of%20S%20Attribute%20State%20Structures) (AttributeBaseDefinition :type Array%20of%20S%20Attribute%20Init%20Row%20Base%20Definition%20Structures))
  ;[0.15 0.15 0.15 0.5] Recive Initial attribute fata from server on client
  (for _array_element AttributeState
    (CallFunction|NotifyAttributeChangeCLIENT _array_element))
  (for _array_element_2 AttributeBaseDefinition
    (Utilities|Map|Add (Variables|Default|GetAttributeDefinitionMap) (.AttributeTag (Utilities|Struct|BreakS_AttributeInitRowBaseDefinition _array_element_2)) _array_element_2)
    (if (GameplayTags|IsGameplayTagValid (.MaxAttributeTag (Utilities|Struct|BreakS_AttributeInitRowBaseDefinition _array_element_2)))
      (Utilities|Map|Add (Variables|Default|GetAttributeDefinitionMap) (.MaxAttributeTag (Utilities|Struct|BreakS_AttributeInitRowBaseDefinition _array_element_2)) _array_element_2))))

(event Custom|NotifyAttributeChange_CLIENT
  (params (AttributeState :type S%20Attribute%20State%20Structure))
  ;[0.15 0.15 0.15 0.5] Handle a single attribute update on tge owning client
  (AttributeSystemNotifier|BroadcastAttributeChanges AttributeState))

(event Custom|InitAndReplicateLoadedData
  ;[0.15 0.15 0.15 0.5] Replicate the freshly initialized attribute data out to connect client
  (bind _values (Utilities|Map|Values (Variables|Default|GetAttributeDefinitionMap)))
  (bind _values_2 (Utilities|Map|Values (Variables|Default|GetAttributeStateMap)))
  (CallFunction|ReplicateInitAttributeDataCLIENT _values_2 _values)
  (for _array_element _values_2
    (AttributeSystemThreshold|UpdateThresholdTagsfromAttribute (.attributetag _array_element)))
  (AttributeSystemLoader|CheckIsAttributeSystemInitialize))

(event Custom|InitializeBaseDefinitionData
  (params (DT%20AttributeBaseValue :type Data%20Table%20Soft%20Object%20Reference))
  (bind _output (Utilities|ResolveSoftReference DT%20AttributeBaseValue))
  ;[0.15 0.15 0.15 0.5] Load base attribute start and max values from the Definition DataTable
  (Utilities|AsyncLoadAsset DT%20AttributeBaseValue
    (:Completed
      (bind _outrownames (DataTable|GetDataTableRowNames _output))
      (for _array_element _outrownames
        (bind _returnvalue (Utilities|GetDataTableRow _output _array_element)
          (:then
            (AttributeSystemLoader|RegistreAttributeTag (.AttributeTag (Utilities|Struct|BreakS_AttributeInitRowBaseDefinition _returnvalue)) _returnvalue (.StartValue (Utilities|Struct|BreakS_AttributeInitRowBaseDefinition _returnvalue)))
            (if (GameplayTags|IsGameplayTagValid (.MaxAttributeTag (Utilities|Struct|BreakS_AttributeInitRowBaseDefinition _returnvalue)))
              (AttributeSystemLoader|RegistreAttributeTag (.MaxAttributeTag (Utilities|Struct|BreakS_AttributeInitRowBaseDefinition _returnvalue)) _returnvalue (.BaseValue (Utilities|Struct|BreakS_AttributeInitRowBaseDefinition _returnvalue)))))))
      (AttributeSystemLoader|CheckIsAttributeSystemInitialize))))

(event Custom|InitializeThresholdData
  (params (DT%20AttributeThreshold :type Data%20Table%20Soft%20Object%20Reference))
  (bind _output (Utilities|ResolveSoftReference DT%20AttributeThreshold))
  ;[0.15 0.15 0.15 0.5] Load All threshold definitions for status tag
  (Utilities|AsyncLoadAsset DT%20AttributeThreshold
    (:Completed
      (bind _outrownames (DataTable|GetDataTableRowNames _output))
      (for _array_element _outrownames
        (bind _returnvalue (Utilities|GetDataTableRow _output _array_element)
          (:then
            (Utilities|Array|Add (Variables|AttributeSystemThreshold|GetAllAttributeThresholdTags) _returnvalue))))
      (AttributeSystemLoader|CheckIsAttributeSystemInitialize))))

(fn RegistreAttributeTag
  (params (AttributeTag :type Gameplay%20Tag%20Structure) (BaseDefinition :type S%20Attribute%20Init%20Row%20Base%20Definition%20Structure) (CurrentValue :type Float%20%28double-precision%29))
  ;[0.15 0.15 0.15 0.5] Register a new attribute
  (Utilities|Map|Add (Variables|Default|GetAttributeDefinitionMap) AttributeTag BaseDefinition)
  (Utilities|Map|Add (Variables|Default|GetAttributeStateMap) AttributeTag (Utilities|Struct|MakeS_AttributeState AttributeTag CurrentValue)))

(fn BroadcastAttributeChanges
  (params (AttributeState :type S%20Attribute%20State%20Structure))
  (bind _attributetag (Utilities|Struct|BreakS_AttributeState AttributeState))
  ;[0.15 0.15 0.15 0.5] Fetch Update Full Attribute State
  (Utilities|Map|Add (Variables|Default|GetAttributeStateMap) _attributetag AttributeState)
  (Default|CallOnAnyAttributeValueChanged (Utilities|Struct|MakeS_AttributeGroupValue _attributetag (AttributeSystemGetter/Setter|GetAttributeValues _attributetag))))

(fn GetAttributeValues
  (params (AttributeTag :type Gameplay%20Tag%20Structure))
  (bind _attributedefinitionmap (Variables|Default|GetAttributeDefinitionMap))
  (bind _value (Utilities|Map|Find _attributedefinitionmap AttributeTag))
  (bind (_attributetag _maxattributetag) (Utilities|Struct|BreakS_AttributeInitRowBaseDefinition _value))
  (if (GameplayTags|IsGameplayTagValid _maxattributetag)
    (return (Utilities|Struct|MakeS_AttributeValue (.CurrentValue (AttributeSystemGetter/Setter|GetAttributeCurrentValue _attributetag)) (.CurrentValue (AttributeSystemGetter/Setter|GetAttributeCurrentValue _maxattributetag)) true))
    (else
      (return (Utilities|Struct|MakeS_AttributeValue (.CurrentValue (AttributeSystemGetter/Setter|GetAttributeCurrentValue AttributeTag)) 0.0 false)))))

(fn GetAttributeCurrentValue
  (params (AttributeTag :type Gameplay%20Tag%20Structure))
  (bind _attributestatemap (Variables|Default|GetAttributeStateMap))
  (bind _value (Utilities|Map|Find _attributestatemap AttributeTag))
  (return (Utilities|Struct|BreakS_AttributeState _value) _value))

(fn SetAttributeInstant
  (params (AttributeTag :type Gameplay%20Tag%20Structure) (ModifierOperator :type E_GE_ModifierOperator%20Enum :default "NewEnumerator0") (EvaluatedValue :type Float%20%28double-precision%29))
  (AttributeSystemModification|AddQueueModifier (Utilities|Array|MakeArray (Utilities|Struct|MakeS_AttributeResolvedModifier "00000000000000000000000000000000" "00000000000000000000000000000000" AttributeTag ModifierOperator EvaluatedValue))))

(fn AddQueueModifier
  (params (Modifiers :type Array%20of%20S%20Attribute%20Resolved%20Modifier%20Structures))
  (Utilities|Array|AppendArray (Variables|AttributeSystemModification|GetQueueModifier) Modifiers)
  (AttributeSystemModification|PocessNexQueuedModifiers))

(fn RecalculateModifiersDirectly
  (params (Modifiers :type Array%20of%20S%20Attribute%20Resolved%20Modifier%20Structures))
  (for _array_element Modifiers
    (bind _clampedattributestate (AttributeSystemModification|ClampAttributeValue (.AttributeTag (Utilities|Struct|BreakS_AttributeResolvedModifier _array_element)) (Utilities|Select :Index (.ModifierOperator (Utilities|Struct|BreakS_AttributeResolvedModifier _array_element)) :NewEnumerator0 (+ (.CurrentValue (AttributeSystemGetter/Setter|GetAttributeCurrentValue (.AttributeTag (Utilities|Struct|BreakS_AttributeResolvedModifier _array_element)))) (.EvaluatedValue (Utilities|Struct|BreakS_AttributeResolvedModifier _array_element))) :NewEnumerator1 (* (.CurrentValue (AttributeSystemGetter/Setter|GetAttributeCurrentValue (.AttributeTag (Utilities|Struct|BreakS_AttributeResolvedModifier _array_element)))) (+ 1.0 (.EvaluatedValue (Utilities|Struct|BreakS_AttributeResolvedModifier _array_element)))) :NewEnumerator2 (Math|Float|SafeDivide (.CurrentValue (AttributeSystemGetter/Setter|GetAttributeCurrentValue (.AttributeTag (Utilities|Struct|BreakS_AttributeResolvedModifier _array_element)))) (.EvaluatedValue (Utilities|Struct|BreakS_AttributeResolvedModifier _array_element))) :NewEnumerator3 (.EvaluatedValue (Utilities|Struct|BreakS_AttributeResolvedModifier _array_element)))))
    (AttributeSystemModification|SetAttributeStateValue _clampedattributestate)))

(fn ClampAttributeValue
  (params (AttributeTag :type Gameplay%20Tag%20Structure) (NewCurrentValue :type Float%20%28double-precision%29))
  (bind _attributedefinitionmap (Variables|Default|GetAttributeDefinitionMap))
  (bind _value (Utilities|Map|Find _attributedefinitionmap AttributeTag))
  (bind (_maxattributetag _minvalue _maxvalue _clampbymaxattributevalue) (Utilities|Struct|BreakS_AttributeInitRowBaseDefinition _value))
  (if (and (GameplayTags|IsGameplayTagValid _maxattributetag) _clampbymaxattributevalue)
    (return (Utilities|Struct|MakeS_AttributeState AttributeTag (Math|Float|Clamp(Float) NewCurrentValue _minvalue (.CurrentValue (AttributeSystemGetter/Setter|GetAttributeCurrentValue _maxattributetag)))))
    (else
      (return (Utilities|Struct|MakeS_AttributeState AttributeTag (Math|Float|Clamp(Float) NewCurrentValue _minvalue _maxvalue))))))

(fn SetAttributeStateValue
  (params (AttributeState :type S%20Attribute%20State%20Structure))
  (bind _attributetag (Utilities|Struct|BreakS_AttributeState AttributeState))
  ;[0.15 0.15 0.15 0.5] Write The new live
  (Utilities|Map|Add (Variables|Default|GetAttributeStateMap) _attributetag AttributeState)
  (AttributeSystemThreshold|UpdateThresholdTagsfromAttribute _attributetag)
  (AttributeSystemNotifier|BroadcastAttributeChanges AttributeState)
  (CallFunction|NotifyAttributeChangeCLIENT AttributeState))

(fn PocessNexQueuedModifiers
  (if (not (or (Variables|AttributeSystemModification|GetIsProccessingModifierQueue) (Utilities|Array|IsEmpty (Variables|AttributeSystemModification|GetQueueModifier))))
    (Variables|AttributeSystemModification|SetIsProccessingModifierQueue true)
    (bind _output_get (LocalVariables|SetToExecuteModifiers (Variables|AttributeSystemModification|GetQueueModifier)))
    (Utilities|Array|Clear (Variables|AttributeSystemModification|GetQueueModifier))
    (AttributeSystemModification|RecalculateModifiersDirectly _output_get)
    (Variables|AttributeSystemModification|SetIsProccessingModifierQueue false)
    (AttributeSystemModification|PocessNexQueuedModifiers)))

(fn UpdateThresholdTagsfromAttribute
  (params (AttributeTag :type Gameplay%20Tag%20Structure))
  ;[0.15 0.15 0.15 0.5] Loop through each threshold definition
  (for _array_element (Variables|AttributeSystemThreshold|GetAllAttributeThresholdTags)
    (if (Utilities|Array|ContainsItem (AttributeSystemModification|GetAttributeGroupTags AttributeTag) (.AttributeTagCurrentValue (Utilities|Struct|BreakS_AttributeThresholdTag _array_element)))
      (if (and (>= (Utilities|Select :Index (.ThresholtType (Utilities|Struct|BreakS_AttributeThresholdTag _array_element)) :NewEnumerator0 (Math|Float|SafeDivide (.current (AttributeSystemGetter/Setter|GetAttributeValues (.AttributeTagCurrentValue (Utilities|Struct|BreakS_AttributeThresholdTag _array_element)))) (.max (AttributeSystemGetter/Setter|GetAttributeValues (.AttributeTagCurrentValue (Utilities|Struct|BreakS_AttributeThresholdTag _array_element))))) :NewEnumerator1 (.current (AttributeSystemGetter/Setter|GetAttributeValues (.AttributeTagCurrentValue (Utilities|Struct|BreakS_AttributeThresholdTag _array_element))))) (.MinValue (Utilities|Struct|BreakS_AttributeThresholdTag _array_element))) (<= (Utilities|Select :Index (.ThresholtType (Utilities|Struct|BreakS_AttributeThresholdTag _array_element)) :NewEnumerator0 (Math|Float|SafeDivide (.current (AttributeSystemGetter/Setter|GetAttributeValues (.AttributeTagCurrentValue (Utilities|Struct|BreakS_AttributeThresholdTag _array_element)))) (.max (AttributeSystemGetter/Setter|GetAttributeValues (.AttributeTagCurrentValue (Utilities|Struct|BreakS_AttributeThresholdTag _array_element))))) :NewEnumerator1 (.current (AttributeSystemGetter/Setter|GetAttributeValues (.AttributeTagCurrentValue (Utilities|Struct|BreakS_AttributeThresholdTag _array_element))))) (.MaxValue (Utilities|Struct|BreakS_AttributeThresholdTag _array_element))))
        (bind _result (Class|BPIAbilitySystemProvider|HasGameplayTag(Message) (Components|GetOwner) (.TagToAdd (Utilities|Struct|BreakS_AttributeThresholdTag _array_element))))
        (if (not _result)
          (Class|BPIAbilitySystemProvider|SetGameplayTag(Message) (Components|GetOwner) (.TagToAdd (Utilities|Struct|BreakS_AttributeThresholdTag _array_element)) true))
        (else
          (bind _result_2 (Class|BPIAbilitySystemProvider|HasGameplayTag(Message) (Components|GetOwner) (.TagToAdd (Utilities|Struct|BreakS_AttributeThresholdTag _array_element))))
          (if _result_2
            (Class|BPIAbilitySystemProvider|SetGameplayTag(Message) (Components|GetOwner) (.TagToAdd (Utilities|Struct|BreakS_AttributeThresholdTag _array_element)) false)))))))

(fn GetAttributeGroupTags
  (params (AttributeTag :type Gameplay%20Tag%20Structure))
  (bind _attributedefinitionmap (Variables|Default|GetAttributeDefinitionMap))
  (bind _value (Utilities|Map|Find _attributedefinitionmap AttributeTag))
  (bind (_attributetag _maxattributetag) (Utilities|Struct|BreakS_AttributeInitRowBaseDefinition _value))
  (return (select (GameplayTags|IsGameplayTagValid _maxattributetag) (Utilities|Array|MakeArray _attributetag _maxattributetag) (Utilities|Array|MakeArray _attributetag))))

(fn AddModifierstoAttribute
  (params (Modifiers :type Array%20of%20S%20Attribute%20Resolved%20Modifier%20Structures))
  (for _array_element Modifiers
    (bind _output_get (LocalVariables|SetNewModifiersGroup (.Value (Utilities|Map|Find (Variables|AttributeSystemModification|GetActivateAttributeModifiers) (.AttributeTag (Utilities|Struct|BreakS_AttributeResolvedModifier _array_element))))))
    (Utilities|FlowControl|Sequence
      (:then_0
        (switch Utilities|FlowControl|Switch|SwitchonE_GE_ModifierOperator (.ModifierOperator (Utilities|Struct|BreakS_AttributeResolvedModifier _array_element))
          (:NewEnumerator0
            (Utilities|Array|AddUnique (.AddModifiers (Utilities|Struct|BreakS_AttributeModifiersOperatorGroup _output_get)) _array_element))
          (:NewEnumerator1
            (Utilities|Array|AddUnique (.MultiplyModifiers (Utilities|Struct|BreakS_AttributeModifiersOperatorGroup _output_get)) _array_element))
          (:NewEnumerator2
            (Utilities|Array|AddUnique (.DivideModifiers (Utilities|Struct|BreakS_AttributeModifiersOperatorGroup _output_get)) _array_element))
          (:NewEnumerator3
            (Utilities|Struct|SetmembersinS_AttributeModifiersOperatorGroup (LocalVariables|GetNewModifiersGroup) (Utilities|Array|MakeArray _array_element)))))
      (:then_1
        (Utilities|Array|AddUnique (LocalVariables|GetModifiedAttributeTags) (.AttributeTag (Utilities|Struct|BreakS_AttributeResolvedModifier _array_element)))
        (Utilities|Map|Add (Variables|AttributeSystemModification|GetActivateAttributeModifiers) (.AttributeTag (Utilities|Struct|BreakS_AttributeResolvedModifier _array_element)) (LocalVariables|GetNewModifiersGroup)))))
  (for _array_element_2 (LocalVariables|GetModifiedAttributeTags)
    (AttributeSystemModification|RecalculateAttribute _array_element_2)))

(fn RecalculateAttribute
  (params (AttributeTag :type Gameplay%20Tag%20Structure))
  (bind _activateattributemodifiers (Variables|AttributeSystemModification|GetActivateAttributeModifiers))
  (bind (_value _returnvalue) (Utilities|Map|Find _activateattributemodifiers AttributeTag))
  (bind (_overridemodifiers _addmodifiers _multiplymodifiers _dividemodifiers) (Utilities|Struct|BreakS_AttributeModifiersOperatorGroup _value))
  ;[0.15 0.15 0.15 0.5] Final Attribute value
  (if _returnvalue
    (bind _clampedattributestate (AttributeSystemModification|ClampAttributeValue AttributeTag (Math|Float|SafeDivide (* (+ (select (Utilities|Array|IsNotEmpty _overridemodifiers) (AttributeSystemModification|SumModifiersValues _overridemodifiers) (AttributeSystemGetter/Setter|GetAttributeBaseValue AttributeTag)) (AttributeSystemModification|SumModifiersValues _addmodifiers)) (+ 1.0 (AttributeSystemModification|SumModifiersValues _multiplymodifiers))) (+ 1.0 (AttributeSystemModification|SumModifiersValues _dividemodifiers)))))
    (AttributeSystemModification|SetAttributeStateValue _clampedattributestate)))

(fn SumModifiersValues
  (params (Modifiers :type Array%20of%20S%20Attribute%20Resolved%20Modifier%20Structures))
  ;[0.15 0.15 0.15 0.5] Iterate all resolved modifiers
  (for _array_element Modifiers
    (LocalVariables|SetTempSum (+ (LocalVariables|GetTempSum) (Utilities|Struct|BreakS_AttributeResolvedModifier _array_element))))
  (return (LocalVariables|GetTempSum)))

(fn GetAttributeBaseValue
  (params (AttributeTag :type Gameplay%20Tag%20Structure))
  ;[0.15 0.15 0.15 0.5] Returns a atrribute BaseValue
  (return (Utilities|Struct|BreakS_AttributeInitRowBaseDefinition (.Value (Utilities|Map|Find (Variables|Default|GetAttributeDefinitionMap) AttributeTag)))))

(fn RemoveModifiersfromAttribute
  (params (GameplayEffectGUID :type Guid%20Structure))
  ;[0.15 0.15 0.15 0.5] Find an remove modifiers
  (bind _keys (Utilities|Map|Keys (Variables|AttributeSystemModification|GetActivateAttributeModifiers)))
  (for _array_element _keys
    (bind _output_get (LocalVariables|SetModifierGroups (.Value (Utilities|Map|Find (Variables|AttributeSystemModification|GetActivateAttributeModifiers) _array_element))))
    (LocalVariables|SetIsModified false)
    (Utilities|FlowControl|Sequence
      (:then_0
        (bind (_ismodified _newmodifiers) (AttributeSystemModification|RemoveModifiersbyEffectGUID (.OverrideModifiers (Utilities|Struct|BreakS_AttributeModifiersOperatorGroup _output_get)) GameplayEffectGUID))
        (if _ismodified
          (Utilities|Struct|SetmembersinS_AttributeModifiersOperatorGroup (LocalVariables|GetModifierGroups) _newmodifiers)
          (LocalVariables|SetIsModified true)))
      (:then_1
        (bind (_ismodified_2 _newmodifiers_2) (AttributeSystemModification|RemoveModifiersbyEffectGUID (.AddModifiers (Utilities|Struct|BreakS_AttributeModifiersOperatorGroup _output_get)) GameplayEffectGUID))
        (if _ismodified_2
          (Utilities|Struct|SetmembersinS_AttributeModifiersOperatorGroup (LocalVariables|GetModifierGroups) _newmodifiers_2)
          (LocalVariables|SetIsModified true)))
      (:then_2
        (bind (_ismodified_3 _newmodifiers_3) (AttributeSystemModification|RemoveModifiersbyEffectGUID (.MultiplyModifiers (Utilities|Struct|BreakS_AttributeModifiersOperatorGroup _output_get)) GameplayEffectGUID))
        (if _ismodified_3
          (Utilities|Struct|SetmembersinS_AttributeModifiersOperatorGroup (LocalVariables|GetModifierGroups) _newmodifiers_3)
          (LocalVariables|SetIsModified true)))
      (:then_3
        (bind (_ismodified_4 _newmodifiers_4) (AttributeSystemModification|RemoveModifiersbyEffectGUID (.DivideModifiers (Utilities|Struct|BreakS_AttributeModifiersOperatorGroup _output_get)) GameplayEffectGUID))
        (if _ismodified_4
          (Utilities|Struct|SetmembersinS_AttributeModifiersOperatorGroup (LocalVariables|GetModifierGroups) _newmodifiers_4)
          (LocalVariables|SetIsModified true)))
      (:then_4
        (if (LocalVariables|GetIsModified)
          (Utilities|Map|Add (Variables|AttributeSystemModification|GetActivateAttributeModifiers) _array_element (LocalVariables|GetModifierGroups))
          (AttributeSystemModification|RecalculateAttribute _array_element))))))

(fn RemoveModifiersbyEffectGUID
  (params (ResolvedModifiers :type Array%20of%20S%20Attribute%20Resolved%20Modifier%20Structures) (GameplayEffectGUID :type Guid%20Structure))
  ;[0.15 0.15 0.15 0.5] Filter attribute
  (LocalVariables|SetModifiers ResolvedModifiers)
  (for _array_element ResolvedModifiers
    (if (== GameplayEffectGUID (Utilities|Struct|BreakS_AttributeResolvedModifier _array_element))
      (Utilities|Array|RemoveItem (LocalVariables|GetModifiers) _array_element)
      (LocalVariables|SetFound true)))
  (return (LocalVariables|GetFound) (LocalVariables|GetModifiers)))

(fn GetAttributeDerivedDefinition
  (params (AttributeDerivedTag :type Gameplay%20Tag%20Structure))
  (bind _attributederiveddefinitionmap (Variables|AttributeSystemDerivedState|GetAttributeDerivedDefinitionMap))
  (bind (_value _returnvalue) (Utilities|Map|Find _attributederiveddefinitionmap AttributeDerivedTag))
  (bind (_modifierratetype _valuesbylevel) (Utilities|Struct|BreakS_AttributeInitRowDerivedStatValue _value))
  (if _returnvalue
    (return _modifierratetype (Utilities|Array|Get(acopy) _valuesbylevel))
    (else
      (CallFunction|PrintError "Attribute derived stat not found for derivedTag" (Utilities|String|ToString(Name) (GameplayTags|GetTagName AttributeDerivedTag)) true)
      (return "NewEnumerator0" 0.0))))

(fn GetAllAttributeTags
  (bind _keys (Utilities|Map|Keys (Variables|Default|GetAttributeStateMap)))
  (return (GameplayTags|MakeGameplayTagContainerfromArray _keys)))

(fn CheckIsAttributeSystemInitialize
  ;[0.15 0.15 0.15 0.5] We trigger FIRST the initialization replicate and fire THEN OnAttributeSystemReady Event.
  (bind _result (Math|Integer|IncrementInt (Variables|AttributeSystemLoader|GetAsyncLoadCounter))
    (:%20%20
      (bind _output_get (Variables|AttributeSystemLoader|SetIsComponentInitialized (>= _result 4)))
      (if _output_get
        (Default|CallOnAttributeSystemIsReady)
        (elif (>= _result 3)
          (CallFunction|InitandReplicateLoadedData))))))

(fn IsAttributeComponetReady
  (return (Variables|AttributeSystemLoader|GetIsComponentInitialized)))