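; Gameplay ability for character sprint that applies a stamina drain once the character is moving.
; On activation it commits, checks whether its logic should execute, then listens for the State.Movement.IsMoving tag.
; If that tag is present, initially or after a change, it applies GE_Drain_Stamina_Sprint to the target ASC.
; Any other listened tag ends the ability when it becomes present.
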(event EventOnAbilityActivated
  ;[0.15 0.15 0.15 0.5] While Sprint is held, the ability listens for the is moving tag and appplies the stamina drain effect once movement starts.
  (bind _successfully (CallFunction|CommitAbility))
  (if _successfully
    (Utilities|ShouldExectureAbilityLogic
      (:Executable
        (Utilities|BindTagListener "(GameplayTags=((TagName=\"State.Movement.IsMoving\"),(TagName=\"Attribute.Status.Stamina.Low\"),(TagName=\"Attribute.Status.Stamina.Empty\")))")
        (Utilities|HasGameplayTag "(TagName=\"State.Movement.IsMoving\")"
          (:true
            (Default|ApplyGameplyEffecttoSelf (CallFunction|GetTargetASCfromContext) "/Game/Core/Blueprints/Systems/AbilitySystem/GameplayEffects/Drain/GE_Drain_Stamina_Sprint.GE_Drain_Stamina_Sprint_C")))))))

(event EventOnTagChanged
  (params (Context :type S%20Gameplay%20Tag%20Changed%20Context%20Structure))
  ;[0.15 0.15 0.15 0.5] While Sprint is held, the ability listens for the is moving tag and appplies the stamina drain effect once movement starts.
  (|SwitchGameplayTag (.tag Context)
    (:Default
      (Utilities|HasGameplayTag (.tag Context)
        (:true
          (CallFunction|EndAbility))))
    (:State.Movement.IsMoving
      (Utilities|HasGameplayTag "(TagName=\"State.Movement.IsMoving\")"
        (:true
          (Default|ApplyGameplyEffecttoSelf (CallFunction|GetTargetASCfromContext) "/Game/Core/Blueprints/Systems/AbilitySystem/GameplayEffects/Drain/GE_Drain_Stamina_Sprint.GE_Drain_Stamina_Sprint_C"))))))