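; GA_ItemUse_Base is a base gameplay ability for using items.
; On activation it commits the ability, then plays its AnimMontage, runs the custom use logic and prints a debug message.
; The montage goes through a multicast, camera-view-aware message on the player character.
; ExecuteCustomUseLogic is a separate event, apparently a hook for child abilities, and only ends the ability here.
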(event Custom|PlayAnimMontage
  (Class|BPICharacter|CharPlayAnimMontagebyCamView(Message) (CallFunction|GetPlayerCharacter) (Variables|Default|GetAnimMontage) true))

(event Custom|ExecuteCustomUseLogic
  (CallFunction|EndAbility))

(event EventOnAbilityActivated
  (bind _successfully (CallFunction|CommitAbility))
  (if _successfully
    (CallFunction|PlayAnimMontage)
    (CallFunction|ExecuteCustomUseLogic)
    (Development|PrintString 0 "Ability used")))