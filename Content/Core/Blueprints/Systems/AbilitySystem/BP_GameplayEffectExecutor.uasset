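; Actor that runs one gameplay effect instance on a target in a Blueprint ability system, driven by its EffectDefinition.
; After an optional delay, it grants or removes tags, evaluates modifiers once, then executes them instantly or periodically, or registers them on the attribute component.
; It destroys itself after instant execution, duration expiry or failed ongoing tag conditions.
; Destruction clears timers, unregisters modifiers by instance GUID and withdraws added tags.
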(event Custom|ApplyEffect
  ;[0.15 0.15 0.15 0.5] Initialization
  (Utilities|FlowControl|Sequence
    (:then_0
      ;;[0.15 0.15 0.15 0.5] Initialize data y event listener
      (bind (_hastags _ongoingtags) (CallFunction|GetListenerRelevantTags))
      (if _hastags
        (bind _gameplaytagscomp (Default|GetGameplayTagsComp (CallFunction|GetTargetASC)))
        (Default|BindTagListener _gameplaytagscomp self _ongoingtags)))
    (:then_1
      ;;[0.15 0.15 0.15 0.5] Start Effect
      (bind (_result _delaytime) (CallFunction|HasImpactDelay))
      (if _result
        (Utilities|FlowControl|Delay _delaytime))
      (CallFunction|ApplyEffectModifiers))))

(event Custom|ApplyEffectModifiers
  ;[0.15 0.15 0.15 0.5] Register Modifiers
  (CallFunction|GrantExecutionTags)
  (CallFunction|ResolveModifiersOnce)
  (switch Utilities|FlowControl|Switch|SwitchonE_GE_DurationPolicy (Variables|/Game/Core/Blueprints/Systems/AbilitySystem/GameplayeEffect_Base.GameplayeEffect_Base_C|GetDurationPolicy (Variables|EffectExecutor|GetEffectDefinition))
    (:NewEnumerator0
      (CallFunction|ExecuteModifiers)
      (CallFunction|EndEffect))
    (:NewEnumerator1
      (if (CallFunction|IsPeriodicEffect) :!label _label
        (CallFunction|StartPeriodTimerLoop)
        (else
          (CallFunction|RegisterModifiers))))
    (:NewEnumerator2
      (bind _returnvalue (Utilities|Time|SetTimerbyEvent (delegate Custom|DurationEnd) (Variables|/Game/Core/Blueprints/Systems/AbilitySystem/GameplayeEffect_Base.GameplayeEffect_Base_C|GetDuration (Variables|EffectExecutor|GetEffectDefinition))))
      (Variables|Internal|SetDurationTimerHandle _returnvalue)
      (goto _label))))

(event Custom|ExecuteModifiers
  ;[0.15 0.15 0.15 0.5] Handle modifiers
  (bind _values (Utilities|Map|Values (Variables|Modifiers|GetActiveResolvedModifiers)))
  (bind _attributesystemcomp (Default|GetAttributeSystemComp (CallFunction|GetTargetASC)))
  (Default|AddQueueModifier _attributesystemcomp _values))

(event Custom|EndEffect
  ;[0.15 0.15 0.15 0.5] Effect end
  (Actor|DestroyActor))

(event Custom|RegisterModifiers
  ;[0.15 0.15 0.15 0.5] Handle modifiers
  (bind _values (Utilities|Map|Values (Variables|Modifiers|GetActiveResolvedModifiers)))
  (bind _attributesystemcomp (Default|GetAttributeSystemComp (CallFunction|GetTargetASC)))
  (Default|AddModifierstoAttribute _attributesystemcomp _values))

(event Custom|UnregisterModifiers
  ;[0.15 0.15 0.15 0.5] Handle modifiers
  (bind _attributesystemcomp (Default|GetAttributeSystemComp (CallFunction|GetTargetASC)))
  (Default|RemoveModifiersfromAttribute _attributesystemcomp (Variables|EffectExecutor|GetEffectInstanceID)))

(event Custom|StartPeriodTimerLoop
  (bind _effectdefinition (Variables|EffectExecutor|GetEffectDefinition))
  ;[0.15 0.15 0.15 0.5] Period executor fo effect
  (if (Variables|/Game/Core/Blueprints/Systems/AbilitySystem/GameplayeEffect_Base.GameplayeEffect_Base_C|GetExecuteEffectOnApplication _effectdefinition)
    (CallFunction|ExecuteModifiers))
  (bind _returnvalue (Utilities|Time|SetTimerbyEvent (delegate Custom|PeriodicRun) (Variables|/Game/Core/Blueprints/Systems/AbilitySystem/GameplayeEffect_Base.GameplayeEffect_Base_C|GetPeriod _effectdefinition) true))
  (Variables|Internal|SetPeriodTimerHandle _returnvalue))

(event Custom|PeriodicRun
  ;[0.15 0.15 0.15 0.5] Period executor fo effect
  (CallFunction|ExecuteModifiers))

(event Custom|DurationEnd
  ;[0.15 0.15 0.15 0.5] Register Modifiers
  (CallFunction|EndEffect))

(event EventDestroyed
  ;[0.15 0.15 0.15 0.5] Effect end
  (Utilities|Time|ClearandInvalidateTimerbyHandle (Variables|Internal|GetPeriodTimerHandle))
  (Utilities|Time|ClearandInvalidateTimerbyHandle (Variables|Internal|GetDurationTimerHandle))
  (CallFunction|RemoveExecutionTags)
  (CallFunction|UnregisterModifiers)
  (bind _gameplaytagscomp (Default|GetGameplayTagsComp (CallFunction|GetTargetASC)))
  (Default|UnbindListenerfromAllTags _gameplaytagscomp self))

(event EventOnTagChanged
  (params (Context :type S%20Gameplay%20Tag%20Changed%20Context%20Structure))
  (bind _effectdefinition (Variables|EffectExecutor|GetEffectDefinition))
  (bind _ongoingrequiredtags (Variables|/Game/Core/Blueprints/Systems/AbilitySystem/GameplayeEffect_Base.GameplayeEffect_Base_C|GetOnGoingRequiredTags _effectdefinition))
  (bind _ongoingblocktags (Variables|/Game/Core/Blueprints/Systems/AbilitySystem/GameplayeEffect_Base.GameplayeEffect_Base_C|GetOnGoingBlockTags _effectdefinition))
  ;[0.15 0.15 0.15 0.5] Event listener for tag
  (if (or (and (CallFunction|IsTagContainerNotEmpty _ongoingrequiredtags) (not (GameplayTags|HasAllTags _ongoingrequiredtags (.activetags Context) true))) (and (CallFunction|IsTagContainerNotEmpty _ongoingblocktags) (GameplayTags|HasAllTags _ongoingblocktags (.activetags Context) true)))
    (CallFunction|EndEffect)))

(fn ConstructionScript
  (Variables|EffectExecutor|SetEffectInstanceID (Guid|NewGuid)))

(fn ResolveModifiersOnce
  (if (== (Utilities|Map|Length (Variables|Modifiers|GetActiveResolvedModifiers)) 0)
    (for _array_element (Variables|/Game/Core/Blueprints/Systems/AbilitySystem/GameplayeEffect_Base.GameplayeEffect_Base_C|GetModifiers (Variables|EffectExecutor|GetEffectDefinition))
      (bind _output_get (LocalVariables|SetPendingModifierGUID (Guid|NewGuid)))
      (Utilities|Map|Add (Variables|Modifiers|GetActiveResolvedModifiers) _output_get (Utilities|Struct|MakeS_AttributeResolvedModifier _output_get (Variables|EffectExecutor|GetEffectInstanceID) (.AttributeTag (Utilities|Struct|BreakS_GameplayEffectAttributeModifier _array_element)) (.ModifiersOperator (Utilities|Struct|BreakS_GameplayEffectAttributeModifier _array_element)) (Default|EvaluateModifierValue (Variables|EffectExecutor|GetEffectDefinition) _array_element))))))

(fn GetTargetASC
  (return (Utilities|Struct|BreakS_GameplayEffectContext (Variables|EffectExecutor|GetExecutionContext))))

(fn IsPeriodicEffect
  (bind _effectdefinition (Variables|EffectExecutor|GetEffectDefinition))
  (return (and (> (Variables|/Game/Core/Blueprints/Systems/AbilitySystem/GameplayeEffect_Base.GameplayeEffect_Base_C|GetPeriod _effectdefinition) 0.0) (Utilities|Enum|NotEqual(Enum) (Variables|/Game/Core/Blueprints/Systems/AbilitySystem/GameplayeEffect_Base.GameplayeEffect_Base_C|GetDurationPolicy _effectdefinition) "NewEnumerator0"))))

(fn HasImpactDelay
  (bind _effectdefinition (Variables|EffectExecutor|GetEffectDefinition))
  (bind _executiondelay (Variables|/Game/Core/Blueprints/Systems/AbilitySystem/GameplayeEffect_Base.GameplayeEffect_Base_C|GetExecutionDelay _effectdefinition))
  (return (> _executiondelay 0.0) _executiondelay))

(fn GrantExecutionTags
  (bind _effectdefinition (Variables|EffectExecutor|GetEffectDefinition))
  (bind _effectdefinition_2 (Variables|EffectExecutor|GetEffectDefinition))
  (bind _grantedtags (Variables|/Game/Core/Blueprints/Systems/AbilitySystem/GameplayeEffect_Base.GameplayeEffect_Base_C|GetGrantedTags _effectdefinition))
  (bind _grantedtags_2 (Variables|/Game/Core/Blueprints/Systems/AbilitySystem/GameplayeEffect_Base.GameplayeEffect_Base_C|GetGrantedTags _effectdefinition_2))
  (bind _remove (Utilities|Struct|BreakS_TagModification _grantedtags))
  (bind _add (Utilities|Struct|BreakS_TagModification _grantedtags_2))
  (bind _gameplaytagscomp (Default|GetGameplayTagsComp (CallFunction|GetTargetASC)))
  (Utilities|FlowControl|Sequence
    (:then_0
      (if (CallFunction|IsTagContainerNotEmpty _add)
        (Default|SetGameplayTags _gameplaytagscomp _add true)))
    (:then_1
      (if (CallFunction|IsTagContainerNotEmpty _remove)
        (Default|SetGameplayTags _gameplaytagscomp _remove false)))))

(fn RemoveExecutionTags
  (bind _gameplaytagscomp (Default|GetGameplayTagsComp (CallFunction|GetTargetASC)))
  (Default|SetGameplayTags _gameplaytagscomp (Utilities|Struct|BreakS_TagModification (Variables|/Game/Core/Blueprints/Systems/AbilitySystem/GameplayeEffect_Base.GameplayeEffect_Base_C|GetGrantedTags (Variables|EffectExecutor|GetEffectDefinition))) false))

(fn GetListenerRelevantTags
  (bind _effectdefinition (Variables|EffectExecutor|GetEffectDefinition))
  (bind _output_get (LocalVariables|SetTags (Variables|/Game/Core/Blueprints/Systems/AbilitySystem/GameplayeEffect_Base.GameplayeEffect_Base_C|GetOnGoingRequiredTags _effectdefinition)))
  (GameplayTags|AppendGameplayTagContainers _output_get (Variables|/Game/Core/Blueprints/Systems/AbilitySystem/GameplayeEffect_Base.GameplayeEffect_Base_C|GetOnGoingBlockTags _effectdefinition))
  (return (CallFunction|IsTagContainerNotEmpty (LocalVariables|GetTags)) (LocalVariables|GetTags)))