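; Equipment component for the player character that spawns a default hands actor on the server and manages the equipped main-hand item.
; Equip requests replace the current item, async-loading and spawning its actor from a soft item data asset, with both-hands items sharing the right-hand slot.
; A client event mirrors the slot map.
; The equipped actor's OnRep broadcasts equip changes, deferring arm pose updates until item data resolves.
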(event Custom|SetEquippedItem_SERVER
  (params (EquipmentSlot :type E_ItemEquipmentSlot%20Enum :default "NewEnumerator0") (ItemDataAsset :type PDA%20Item%20Data%20Soft%20Object%20Reference))
  ;[0.15 0.15 0.15 0.5] MainEquipment event call
  (switch Utilities|FlowControl|Switch|SwitchonE_ItemEquipmentSlot EquipmentSlot
    (:NewEnumerator1
      _)
    (:NewEnumerator2
      _))
  (CallFunction|UnequipMainHadItem "NewEnumerator1")
  (CallFunction|SpawnMainHandItem "NewEnumerator1" ItemDataAsset))

(event Custom|OnRep_EquippedItemActor_Event
  ;[0.15 0.15 0.15 0.5] Wait for ItemDataComponent to be resolved before applying arm pose or equipment logic.
  ; The OnltemDataResolved event ensures that all Item Data references are fully loaded and ready before continuing the setup flow
  (bind _equippeditemactor (Variables|Default|GetEquippedItemActor)
    (:then
      (Default|CallOnMainHandEquipped _equippeditemactor)
      (bind _itemdatacomp (Class|BPIItemMaster|GetItemDataComp(Message) _equippeditemactor))
      (bind _itemdata (Class|BPIItemData|GetItemData(Message) _itemdatacomp))
      (Utilities|IsValid _itemdata
        (:Is%20Valid
          (CallFunction|OnItemDataResolvedEvent))
        (:Is%20Not%20Valid
          (EventDispatchers|AssignOnItemDataResolved _itemdatacomp (delegate Custom|OnItemDataResolved_Event)))))
    (:else
      (Default|CallOnMainHandUnequipped))))

(event Custom|SetEquipmentSlotAsset_CLIENT
  (params (EquipmentSlot :type E_ItemEquipmentSlot%20Enum%20%28by%20ref%29 :default "NewEnumerator0") (ItemDataAsset :type PDA%20Item%20Data%20Soft%20Object%20Reference%20%28by%20ref%29))
  ;[0.15 0.15 0.15 0.5] Replicate the EquipmentSlot Map to the client
  (Utilities|Map|Add (Variables|Default|GetEquipmentSlot) EquipmentSlot ItemDataAsset))

(event Custom|SetEquipmentSlotAsset
  (params (EquipmentSlot :type E_ItemEquipmentSlot%20Enum%20%28by%20ref%29 :default "NewEnumerator0") (ItemDataAsset :type PDA%20Item%20Data%20Soft%20Object%20Reference%20%28by%20ref%29))
  ;[0.15 0.15 0.15 0.5] Replicate the EquipmentSlot Map to the client
  (Utilities|Map|Add (Variables|Default|GetEquipmentSlot) EquipmentSlot ItemDataAsset)
  (CallFunction|SetEquipmentSlotAssetCLIENT "NewEnumerator0"))

(event Custom|SpawnMainHandItem
  (params (EquipmentSlot :type E_ItemEquipmentSlot%20Enum :default "NewEnumerator0") (ItemDataAsset :type PDA%20Item%20Data%20Soft%20Object%20Reference))
  ;[0.15 0.15 0.15 0.5] Handle MainHand Equipment
  (if (Utilities|IsValidSoftObjectReference ItemDataAsset)
    (bind _itemdata (CallFunction|ResolveSoftItemDataReference ItemDataAsset))
    (bind _returnvalue (Class|BPIItemData|IsEquippable(Message) _itemdata))
    (if _returnvalue
      (CallFunction|SetEquipmentSlotAsset EquipmentSlot ItemDataAsset)
      (bind _playercharacter (Class|BPICharacter|GetBpPlayerCharacter(Message) (Components|GetOwner)))
      (Utilities|AsyncLoadClassAsset (Variables|/Game/Core/Blueprints/PrimaryDataAssets/PDA_ItemData.PDA_ItemData_C|GetEquipActorClass _itemdata)
        (:Completed
          (bind _returnvalue_2 (Game|SpawnActorfromClass (Utilities|ResolveSoftReference (Variables|/Game/Core/Blueprints/PrimaryDataAssets/PDA_ItemData.PDA_ItemData_C|GetEquipActorClass _itemdata)) (Math|Transform|MakeTransform "0, 0, 0" "0, 0, 0" "1.000000,1.000000,1.000000") "AlwaysSpawn" "MultiplyWithRoot" _playercharacter ItemDataAsset _playercharacter))
          (Variables|Default|SetEquippedItemActor _returnvalue_2))))))

(event Custom|OnItemDataResolved_Event
  ;[0.15 0.15 0.15 0.5] Wait for ItemDataComponent to be resolved before applying arm pose or equipment logic.
  ; The OnltemDataResolved event ensures that all Item Data references are fully loaded and ready before continuing the setup flow
  (bind (_armposesetasset _attachsocket) (EquipamentComponent|GetEquippedMainHandArmPoseSet))
  (Default|CallOnArmPoseSetChang _armposesetasset _attachsocket))

(event EventBeginPlay
  ;[0.15 0.15 0.15 0.5] Handles spawning the default hands at the start of the game. The hands are always present in the game world and serve as the default equipped item for interaction or basic
  ; harvesting. They should not be confused with tools like the axe or pickaxe, which are separate equippable items,
  ; The short delay of 0.5 seconds ensures that both the Ability System and all character components are fully initialized on the server before spawning the default hands actor.
  ; This prevents potential timing issues during startup where references might not yet be valid.
  (Networking|SwitchHasAuthority
    (:Authority
      (Utilities|FlowControl|Delay 0.5)
      (bind _playercharacter (Class|BPICharacter|GetBpPlayerCharacter(Message) (Components|GetOwner)))
      (bind _returnvalue (Game|SpawnActorfromClass "/Game/Core/Blueprints/Items/Equippable/Hands/BP_ItemEquippableHands.BP_ItemEquippableHands_C" (Math|Transform|MakeTransform "0, 0, 0" "0, 0, 0" "1.000000,1.000000,1.000000") "Undefined" "MultiplyWithRoot" _playercharacter "/Game/Core/DataAssets/Items/Equippable/Hands/DA_ItemHands.DA_ItemHands" _playercharacter))
      (Variables|Default|SetEquippedHandsActor _returnvalue))))

(event EventEndPlay
  (params (EndPlayReason :type EEndPlayReason%20Enum :default "Destroyed"))
  ;[0.15 0.15 0.15 0.5] If Player disconnect, cleanup equipments
  (Utilities|FlowControl|Sequence
    (:then_0
      (Networking|SwitchHasAuthority
        (:Authority
          (switch Utilities|FlowControl|Switch|SwitchonEEndPlayReason EndPlayReason
            (:Destroyed
              (CallFunction|UnequipMainHadItem "NewEnumerator1")
              (CallFunction|UnequipHandsActor))))))
    (:then_1
      (EventDispatchers|UnbindallEventsfromOnMainHandEquipped)
      (EventDispatchers|UnbindallEventsfromOnMainHandUnequipped)
      (EventDispatchers|UnbindallEventsfromOnArmPoseSetChang))))

(fn OnRepEquippedItemActor
  (CallFunction|OnRepEquippedItemActorEvent))

(fn IsMainHandEquipped
  (Variables|Default|GetEquippedItemActor
    (:then
      (return true))
    (:else
      (return false))))

(fn UnequipMainHadItem
  (params (EquipmentSlot :type E_ItemEquipmentSlot%20Enum :default "NewEnumerator0"))
  (bind _equippeditemactor (Variables|Default|GetEquippedItemActor)
    (:then
      (Actor|DestroyActor _equippeditemactor)
      (Variables|Default|SetEquippedItemActor 0)
      (CallFunction|SetEquipmentSlotAsset EquipmentSlot))
    (:else)))

(fn GetEquippedMainHandActor
  (return (Variables|Default|GetEquippedItemActor)))

(fn GetEquippedSlotItemDataAsset
  (params (EquipmentSlot :type E_ItemEquipmentSlot%20Enum :default "NewEnumerator0"))
  (bind _value (Utilities|Map|Find (Variables|Default|GetEquipmentSlot) EquipmentSlot))
  (return (Utilities|IsValidSoftObjectReference _value) _value))

(fn GetEquippedMainHandArmPoseSet
  (bind _equippeditemactor (Variables|Default|GetEquippedItemActor)
    (:then
      (bind _itemdatacomp (Default|GetItemDataComp _equippeditemactor))
      (bind (_isequippable _itemequippableinfo) (Class|BPIItemData|GetEquippableInfo(Message) _itemdatacomp))
      (if _isequippable
        (return (.ArmPoseSetAsset (Utilities|Struct|BreakS_ItemEquippableRow _itemequippableinfo)) (.AttachSocket (Utilities|Struct|BreakS_ItemEquippableRow _itemequippableinfo)))
        (else
          _)))
    (:else
      _))
  (return "/Game/Core/DataAssets/ArmPoseSets/DA_ArmPoseSet_Unarmed.DA_ArmPoseSet_Unarmed" "NewEnumerator0"))

(fn GetHandIK
  (bind _equippeditemactor (Variables|Default|GetEquippedItemActor)
    (:then
      (bind (_hashandik _lefthandiktransform _righthandiktransform) (Class|BPIItemEquippable|GetHandIKTransform(Message) _equippeditemactor))
      (return _hashandik _lefthandiktransform _righthandiktransform))
    (:else)))

(fn GetEquippedHandsActor
  (return (Variables|Default|GetEquippedHandsActor)))

(fn UnequipHandsActor
  (bind _equippedhandsactor (Variables|Default|GetEquippedHandsActor)
    (:then
      (Actor|DestroyActor _equippedhandsactor)
      (Variables|Default|SetEquippedHandsActor 0))
    (:else)))