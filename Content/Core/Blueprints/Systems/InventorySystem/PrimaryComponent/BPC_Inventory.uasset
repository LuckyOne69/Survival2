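; Replicated inventory component that manages a fixed set of item slots on its owning actor.
; Server events handle adding with stack overflow, range-checked transfers that merge or swap slots between inventories, and sorting by name, type, weight or quantity.
; Slot writes fire change events on the server and forward them to clients.
; Optional weight totals recalculate after a debounced slot change and broadcast through OnRep; hand-written swap sorts toggle direction and reindex slots.
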(event Custom|SetupSlots_SERVER
  (params (MaxSlotCount :type Integer))
  ;[0.15 0.15 0.15 0.5] Setup Inventory Slots
  (bind _output_get (Variables|InventorySettings|SetMaxSlotCount MaxSlotCount))
  (for _index (range 0 (- _output_get 1))
    (Utilities|Array|Add (Variables|Default|GetInventorySlots) (Utilities|Struct|MakeS_InventorySlot _index self))))

(event Custom|AddItem_SERVER
  (params (Item :type S%20Inventory%20Slot%20Structure))
  ;[0.15 0.15 0.15 0.5] AddItem
  (bind _succesfully (CallFunction|AddItem Item))
  (if _succesfully
    (CallFunction|NotifyItemAddedCLIENT Item)))

(event Custom|TransferItem_SERVER
  (params (ToInventoryComponent :type BPC%20Inventory%20Object%20Reference) (FromIndex :type Integer) (ToIndex :type Integer))
  ;[0.15 0.15 0.15 0.5] Transfer Item
  (Transfer|TransferItem ToInventoryComponent FromIndex ToIndex))

(event Custom|NotifySlotChange_CLIENT
  (params (Slot :type S%20Inventory%20Slot%20Structure))
  ;[0.15 0.15 0.15 0.5] Event Replication
  (Default|CallOnSlotChanged Slot))

(event Custom|CalculateWeight_Event
  (params (Slot :type S%20Inventory%20Slot%20Structure))
  ;[0.15 0.15 0.15 0.5] Calculate Weight
  (Utilities|FlowControl|RetriggerableDelay 0.1)
  (Weight|CalculateTotalWeight))

(event Custom|SortItemsBy_SERVER
  (params (SortBy :type E_SortItemBy%20Enum :default "NewEnumerator0"))
  (bind _currentsortascending (Sort|GetSortAscending SortBy))
  ;[0.15 0.15 0.15 0.5] Sort Items
  (switch Utilities|FlowControl|Switch|SwitchonE_SortItemBy SortBy
    (:NewEnumerator0
      (Sort|SortItemsbyString SortBy _currentsortascending :!label _label))
    (:NewEnumerator1
      (goto _label))
    (:NewEnumerator2
      (Sort|SortItemsbyNumeric SortBy _currentsortascending :!label _label_2))
    (:NewEnumerator3
      (goto _label_2))))

(event Custom|NotifyItemAdded_CLIENT
  (params (Item :type S%20Inventory%20Slot%20Structure))
  ;[0.15 0.15 0.15 0.5] Event Replication
  (Default|CallOnItemAdded Item))

(event EventBeginPlay
  ;[0.15 0.15 0.15 0.5] Init Inventory on Server
  (Networking|SwitchHasAuthority
    (:Authority
      (CallFunction|SetupSlotsSERVER (Variables|InventorySettings|GetMaxSlotCount))
      ;[0.15 0.15 0.15 0.5] Calculate Weight
      (if (Variables|InventorySettings|GetEnableWeightSystem)
        (EventDispatchers|BindEventtoOnSlotChanged (delegate Custom|CalculateWeight_Event))))))

(event EventEndPlay
  (params (EndPlayReason :type EEndPlayReason%20Enum :default "Destroyed"))
  ;[0.15 0.15 0.15 0.5] Init Inventory on Server
  (EventDispatchers|UnbindallEventsfromOnItemAdded)
  (EventDispatchers|UnbindallEventsfromOnWeightChange)
  ;[0.15 0.15 0.15 0.5] Calculate Weight
  (EventDispatchers|UnbindallEventsfromOnSlotChanged))

(fn AddItem
  (params (ItemToAdd :type S%20Inventory%20Slot%20Structure))
  (if (Transfer|IsSlotItemAllowed ItemToAdd)
    (Variables|Sort|SetCurrentSortAscending true)
    (bind _output_get (LocalVariables|SetCurrentItemToAdd ItemToAdd))
    (bind _returnvalue (Utilities|LoadAssetBlocking (Utilities|Struct|BreakS_InventorySlot _output_get)))
    (bind (_isstackable _stacksize) (Class|BPIItemData|GetStackableInfo(Message) _returnvalue))
    (LocalVariables|SetItemStackSize _stacksize)
    (if _isstackable
      ;[0.15 0.15 0.15 0.5] Add Item if same item y has space for staking
      (for _array_element (Variables|Default|GetInventorySlots)
        (bind _output_get_2 (LocalVariables|SetTargetSlot _array_element))
        (if (CallFunction|IsStackeableandHaveSpace _output_get_2 (LocalVariables|GetCurrentItemToAdd))
          (bind _output_get_3 (LocalVariables|SetNewQuantityFromTargetSlot (+ (Utilities|Struct|BreakS_InventorySlot _array_element) (Utilities|Struct|BreakS_InventorySlot (LocalVariables|GetCurrentItemToAdd)))))
          (if (> _output_get_3 (LocalVariables|GetItemStackSize))
            (Getter/Setter|SetQuantityatSlot (LocalVariables|GetTargetSlot) (LocalVariables|GetItemStackSize))
            (Utilities|Struct|SetmembersinS_InventorySlot (LocalVariables|GetCurrentItemToAdd) (- (LocalVariables|GetNewQuantityFromTargetSlot) (LocalVariables|GetItemStackSize)))
            (else
              (Getter/Setter|SetQuantityatSlot (LocalVariables|GetTargetSlot) (LocalVariables|GetNewQuantityFromTargetSlot))
              (return true))))))
    ;[0.15 0.15 0.15 0.5] Add item to enty slot
    (bind (_result _slot) (Search|FindEmptySlot :!label _label))
    (if _result
      (LocalVariables|SetTargetSlot _slot)
      (if (<= (Utilities|Struct|BreakS_InventorySlot (LocalVariables|GetCurrentItemToAdd)) (LocalVariables|GetItemStackSize))
        (Getter/Setter|SetItem (LocalVariables|GetTargetSlot) (LocalVariables|GetCurrentItemToAdd) false)
        (return true)
        (else
          (bind _output_get_4 (LocalVariables|SetTemporaryCacheItemToAdd (LocalVariables|GetCurrentItemToAdd)))
          (bind _structout (Utilities|Struct|SetmembersinS_InventorySlot _output_get_4 (LocalVariables|GetItemStackSize)))
          (Getter/Setter|SetItem (LocalVariables|GetTargetSlot) _structout false)
          (Utilities|Struct|SetmembersinS_InventorySlot (LocalVariables|GetCurrentItemToAdd) (- (Utilities|Struct|BreakS_InventorySlot (LocalVariables|GetCurrentItemToAdd)) (LocalVariables|GetItemStackSize)))
          (goto _label)))
      (else
        (Development|PrintString "TODO: Inventory Is Full")
        (return false)))
    (else
      (return false))))

(fn FindEmptySlot
  (for _array_element (Variables|Default|GetInventorySlots)
    (if (CallFunction|IsSlotEmpty _array_element)
      (return true _array_element)))
  (return false ""))

(fn SetItem
  (params (TargetSlot :type S%20Inventory%20Slot%20Structure) (Item :type S%20Inventory%20Slot%20Structure) (Silent :type Boolean))
  (bind _slotindex (Utilities|Struct|BreakS_InventorySlot TargetSlot))
  (Utilities|Array|SetArrayElem (Variables|Default|GetInventorySlots) _slotindex Item)
  (bind _structout (Utilities|Struct|SetmembersinS_InventorySlot (Utilities|Array|Get(acopy) (Variables|Default|GetInventorySlots) _slotindex) _slotindex self))
  (if (not Silent)
    (Replication|NotifySlotChange _structout)))

(fn NotifySlotChange
  (params (Slot :type S%20Inventory%20Slot%20Structure))
  (Default|CallOnSlotChanged Slot) ; Server Side
  (CallFunction|NotifySlotChangeCLIENT Slot))

(fn SetQuantityatSlot
  (params (TargetSlot :type S%20Inventory%20Slot%20Structure%20%28by%20ref%29) (Quantity :type Integer))
  (bind _inventoryslots (Variables|Default|GetInventorySlots))
  (bind _slotindex (Utilities|Struct|BreakS_InventorySlot TargetSlot))
  (bind _output (Utilities|Array|Get(acopy) _inventoryslots _slotindex))
  (if (== Quantity 0)
    (Transfer|RemoveItematIndex _slotindex)
    (return _output)
    (else
      (bind _structout (Utilities|Struct|SetmembersinS_InventorySlot _output Quantity))
      (Replication|NotifySlotChange _structout)
      (return _structout))))

(fn TransferItem
  (params (ToInventoryComponent :type BPC%20Inventory%20Object%20Reference) (FromIndex :type Integer) (ToIndex :type Integer))
  (bind (_isvalid _slot) (Getter/Setter|GetSlotatIndex FromIndex))
  (if (and (== self ToInventoryComponent) (== FromIndex ToIndex))
    (CallFunction|PrintError "Error: Same Inventory container y same SlotIndex" "" false)
    (else
      (Variables|Sort|SetCurrentSortAscending true)
      (if (Math|Boolean|ANDBoolean (Utilities|IsValid ToInventoryComponent) (Transfer|IsinTransferRange ToInventoryComponent) _isvalid (or (.IsValid (Getter/Setter|GetSlotatIndex ToInventoryComponent ToIndex)) (== ToIndex -1)))
        (if (== ToIndex -1)
          ;[0.15 0.15 0.15 0.5] Transfer item
          (bind _succesfully (CallFunction|AddItem ToInventoryComponent _slot))
          (if _succesfully
            (bind _succesfully_2 (Transfer|RemoveItematIndex FromIndex))
            (return _succesfully_2)
            (else
              (return false)))
          (else
            (bind (_succesfully_3 _allitemsadded) (Transfer|AddItemtoIndex ToInventoryComponent ToIndex _slot))
            (if _succesfully_3
              (if _allitemsadded
                (bind _succesfully_4 (Transfer|RemoveItematIndex FromIndex))
                (return _succesfully_4)
                (else
                  (return false)))
              (else
                (return false)))))
        (else
          _))))
  (return false))

(fn IsinTransferRange
  (params (ToInventoryComponent :type BPC%20Inventory%20Object%20Reference))
  (return (<= (Math|Vector|Distance(Vector) (Transformation|GetActorLocation (Components|GetOwner ToInventoryComponent)) (Transformation|GetActorLocation (Components|GetOwner self))) (Variables|InventorySettings|GetMaxTransferItemDistance))))

(fn GetSlotatIndex
  (params (Index :type Integer))
  (if (Utilities|Array|IsValidIndex (Variables|Default|GetInventorySlots) Index)
    (return true (Utilities|Array|Get(acopy) (Variables|Default|GetInventorySlots) Index))
    (else
      (return false ""))))

(fn RemoveItematIndex
  (params (Index :type Integer))
  (bind (_isvalid _slot) (Getter/Setter|GetSlotatIndex Index))
  (if _isvalid
    (Getter/Setter|SetItem _slot (Utilities|Struct|MakeS_InventorySlot) false)
    (return false)
    (else
      (return false))))

(fn AddItemtoIndex
  (params (TargetIndex :type Integer) (ItemSlotDataToAdd :type S%20Inventory%20Slot%20Structure%20%28by%20ref%29))
  (bind (_isvalid _slot) (Getter/Setter|GetSlotatIndex TargetIndex))
  (if (Transfer|IsSlotItemAllowed ItemSlotDataToAdd)
    (if _isvalid
      (if (CallFunction|IsSlotEmpty _slot)
        (Getter/Setter|SetItem _slot ItemSlotDataToAdd false)
        (return true true)
        (else
          (bind _allitemstacked (Transfer|StackItemonTransfer _slot ItemSlotDataToAdd))
          (return true _allitemstacked)))
      (else
        _)))
  (return false false))

(fn StackItemonTransfer
  (params (TargetSlot :type S%20Inventory%20Slot%20Structure%20%28by%20ref%29) (FromSlot :type S%20Inventory%20Slot%20Structure%20%28by%20ref%29))
  (bind (_quantity _itemdataassets) (Utilities|Struct|BreakS_InventorySlot TargetSlot))
  (if (CallFunction|IsStackeableandHaveSpace TargetSlot FromSlot) ; Slot Found y Item is same y have space y is stackeable
    (bind _returnvalue (Utilities|LoadAssetBlocking _itemdataassets))
    (bind _stacksize (Class|BPIItemData|GetStackableInfo(Message) _returnvalue))
    (LocalVariables|SetItemStackSize _stacksize)
    (bind _output_get (LocalVariables|SetNewQuantityFromTargetSlot (+ _quantity (Utilities|Struct|BreakS_InventorySlot FromSlot))))
    (if (> _output_get (LocalVariables|GetItemStackSize))
      (Getter/Setter|SetQuantityatSlot TargetSlot (LocalVariables|GetItemStackSize))
      (Getter/Setter|SetQuantityatSlot (Utilities|Struct|BreakS_InventorySlot FromSlot) FromSlot (- (LocalVariables|GetNewQuantityFromTargetSlot) (LocalVariables|GetItemStackSize)))
      (return false)
      (else
        (Getter/Setter|SetQuantityatSlot TargetSlot (LocalVariables|GetNewQuantityFromTargetSlot))
        (return true)))
    (else
      (Transfer|SwapIndexes TargetSlot FromSlot)
      (return false))))

(fn SwapIndexes
  (params (Slot :type S%20Inventory%20Slot%20Structure%20%28by%20ref%29) (SwapWithSlot :type S%20Inventory%20Slot%20Structure%20%28by%20ref%29))
  (Getter/Setter|SetItem Slot SwapWithSlot false)
  (Getter/Setter|SetItem (Utilities|Struct|BreakS_InventorySlot SwapWithSlot) SwapWithSlot Slot false))

(fn CalculateTotalWeight
  (for _array_element (Variables|Default|GetInventorySlots)
    (if (not (CallFunction|IsSlotEmpty _array_element))
      (LocalVariables|SetNewTotalWeight (+ (LocalVariables|GetNewTotalWeight) (CallFunction|GetSlotWeight _array_element)))))
  (if (!= (LocalVariables|GetNewTotalWeight) (Variables|Weight|GetTotalWeight))
    (Variables|Weight|SetTotalWeight (LocalVariables|GetNewTotalWeight)))
  (return))

(fn OnRepTotalWeight
  (Default|CallOnWeightChange (Variables|Weight|GetTotalWeight)))

(fn IsSlotItemAllowed
  (params (Slot :type S%20Inventory%20Slot%20Structure%20%28by%20ref%29))
  (bind _alloweditemtype (Variables|InventorySettings|GetAllowedItemType))
  (return (or (Utilities|Array|IsEmpty _alloweditemtype) (Utilities|Array|ContainsItem _alloweditemtype (Utilities|Struct|BreakS_InventorySlot Slot)))))

(fn SortItemsbyNumeric
  (params (SortBy :type E_SortItemBy%20Enum :default "NewEnumerator0") (AscendingSortOrder :type Boolean))
  (switch Utilities|FlowControl|Switch|SwitchonE_SortItemBy SortBy
    (:NewEnumerator0
      (CallFunction|PrintError "Order is not supported by" (Utilities|String|EnumtoString SortBy) true :!label _label))
    (:NewEnumerator1
      (goto _label))
    (:NewEnumerator2
      (for _index (range 1 (Utilities|Array|LastIndex (Variables|Default|GetInventorySlots))) :!label _label_2
        (bind _output_get (LocalVariables|SetIndexCounter _index))
        (while (> _output_get 0)
          (if (select AscendingSortOrder (not (Utilities|Select :Index SortBy :NewEnumerator0 false :NewEnumerator1 false :NewEnumerator2 (> (CallFunction|GetSlotWeight (Utilities|Array|Get(acopy) (Variables|Default|GetInventorySlots) (LocalVariables|GetIndexCounter))) (CallFunction|GetSlotWeight (Utilities|Array|Get(acopy) (Variables|Default|GetInventorySlots) (- (LocalVariables|GetIndexCounter) 1)))) :NewEnumerator3 (> (Utilities|Struct|BreakS_InventorySlot (Utilities|Array|Get(acopy) (Variables|Default|GetInventorySlots) (LocalVariables|GetIndexCounter))) (Utilities|Struct|BreakS_InventorySlot (Utilities|Array|Get(acopy) (Variables|Default|GetInventorySlots) (- (LocalVariables|GetIndexCounter) 1)))))) (Utilities|Select :Index SortBy :NewEnumerator0 false :NewEnumerator1 false :NewEnumerator2 (> (CallFunction|GetSlotWeight (Utilities|Array|Get(acopy) (Variables|Default|GetInventorySlots) (LocalVariables|GetIndexCounter))) (CallFunction|GetSlotWeight (Utilities|Array|Get(acopy) (Variables|Default|GetInventorySlots) (- (LocalVariables|GetIndexCounter) 1)))) :NewEnumerator3 (> (Utilities|Struct|BreakS_InventorySlot (Utilities|Array|Get(acopy) (Variables|Default|GetInventorySlots) (LocalVariables|GetIndexCounter))) (Utilities|Struct|BreakS_InventorySlot (Utilities|Array|Get(acopy) (Variables|Default|GetInventorySlots) (- (LocalVariables|GetIndexCounter) 1))))))
            (Utilities|Array|Swap (Variables|Default|GetInventorySlots) (LocalVariables|GetIndexCounter) (- (LocalVariables|GetIndexCounter) 1))
            (Math|Integer|DecrementInt (LocalVariables|GetIndexCounter))
            (else
              (Math|Integer|DecrementInt (LocalVariables|GetIndexCounter))))))
      (Sort|FixSlotIndex true))
    (:NewEnumerator3
      (goto _label_2)))
  (return))

(fn FixSlotIndex
  (params (CleanEmptySlots :type Boolean))
  (if CleanEmptySlots
    ;[0.15 0.15 0.15 0.5] Clean empty slot
    (for (_array_element _array_index) (Variables|Default|GetInventorySlots)
      (if (not (CallFunction|IsSlotEmpty _array_element))
        (Utilities|Array|Swap (Variables|Default|GetInventorySlots) _array_index (LocalVariables|GetIndex))
        (Math|Integer|IncrementInt (LocalVariables|GetIndex)))))
  (for (_ _array_index_2) (Variables|Default|GetInventorySlots)
    (bind _structout (Utilities|Struct|SetmembersinS_InventorySlot (Utilities|Array|Get(acopy) (Variables|Default|GetInventorySlots) _array_index_2) _array_index_2))
    (Replication|NotifySlotChange _structout)))

(fn SortItemsbyString
  (params (SortBy :type E_SortItemBy%20Enum :default "NewEnumerator0") (AscendingSortOrder :type Boolean))
  (bind _arraytosortstring (LocalVariables|GetArrayToSortString))
  (switch Utilities|FlowControl|Switch|SwitchonE_SortItemBy SortBy
    (:NewEnumerator0
      _)
    (:NewEnumerator1
      _)
    (:NewEnumerator2
      (CallFunction|PrintError "Sort is not supported by" (Utilities|String|EnumtoString SortBy) true :!label _label)
      (return))
    (:NewEnumerator3
      (goto _label)))
  (for (_array_element _array_index) (Variables|Default|GetInventorySlots)
    ;[0.15 0.15 0.15 0.5] Generated a temporary array to sort items by string
    (if (CallFunction|IsSlotNotEmpty _array_element)
      (bind _itemdata (CallFunction|ResolveSoftItemDataReference (Utilities|Struct|BreakS_InventorySlot _array_element)))
      (Utilities|Array|SetArrayElem (LocalVariables|GetArrayToSortString) _array_index (Utilities|Select :Index SortBy :NewEnumerator0 (Utilities|String|ToString(Text) (Variables|/Game/Core/Blueprints/PrimaryDataAssets/PDA_ItemData.PDA_ItemData_C|GetName _itemdata)) :NewEnumerator1 (Utilities|String|ToString(Name) (Variables|/Game/Core/Blueprints/PrimaryDataAssets/PDA_ItemData.PDA_ItemData_C|GetItemID _itemdata)) :NewEnumerator2 "" :NewEnumerator3 "") true)))
  (for (_array_element_2 _array_index_2) (LocalVariables|GetArrayToSortString)
    (for _index (range _array_index_2 (Utilities|Array|LastIndex _arraytosortstring))
      (bind _index_2 (Utilities|FlowControl|ForLoopwithBreak 0 (- (select (> (Utilities|String|Len (Utilities|Array|Get(acopy) _arraytosortstring _index)) (Utilities|String|Len _array_element_2)) (Utilities|String|Len _array_element_2) (Utilities|String|Len (Utilities|Array|Get(acopy) _arraytosortstring _index))) 1) :!label _label_2)
        (:LoopBody
          (if (!= (Utilities|String|GetCharacterasNumber (Utilities|Array|Get(acopy) _arraytosortstring _index) _index_2) (Utilities|String|GetCharacterasNumber _array_element_2 _index_2))
            (goto _label_2 Break)))
        (:Completed
          (if AscendingSortOrder
            (if (> (Utilities|String|GetCharacterasNumber (Utilities|Array|Get(acopy) _arraytosortstring _index) _index_2) (Utilities|String|GetCharacterasNumber _array_element_2 _index_2))
              (Utilities|Array|Swap (LocalVariables|GetArrayToSortString) _index _array_index_2 :!label _label_3)
              (Utilities|Array|Swap (Variables|Default|GetInventorySlots) _index _array_index_2))
            (elif (< (Utilities|String|GetCharacterasNumber (Utilities|Array|Get(acopy) _arraytosortstring _index) _index_2) (Utilities|String|GetCharacterasNumber _array_element_2 _index_2))
              (goto _label_3)))))))
  (Sort|FixSlotIndex true)
  (return))

(fn GetSortAscending
  (params (SortBy :type E_SortItemBy%20Enum :default "NewEnumerator0"))
  (if (Utilities|Enum|NotEqual(Enum) SortBy (Variables|Sort|GetLastSortBy))
    (Variables|Sort|SetCurrentSortAscending false)
    (else
      (Variables|Sort|SetCurrentSortAscending (not (Variables|Sort|GetCurrentSortAscending)))))
  (Variables|Sort|SetLastSortBy SortBy)
  (return (Variables|Sort|GetCurrentSortAscending)))

(fn SubstractItematIndex
  (params (SlotIndex :type Integer) (AmountToRemove :type Integer))
  (bind (_isvalid _slot) (Getter/Setter|GetSlotatIndex SlotIndex))
  (if (and _isvalid (<= AmountToRemove (Utilities|Struct|BreakS_InventorySlot _slot)))
    (bind _unremovedamount (Substract(Remove)Items|SubstractQuantityatSlot (Utilities|Array|Get(acopy) (Variables|Default|GetInventorySlots) SlotIndex) AmountToRemove))
    (if (== _unremovedamount 0)
      _
      (else
        (CallFunction|PrintError "After removing the item from the slot an amount remaints Something is wrong." (Utilities|String|ToString(Integer) _unremovedamount) true)))
    (return true)
    (else
      (return false))))

(fn SubstractQuantityatSlot
  (params (TargetSlot :type S%20Inventory%20Slot%20Structure) (AmountToRemove :type Integer))
  (bind _quantity (Utilities|Struct|BreakS_InventorySlot TargetSlot))
  (LocalVariables|SetLocalQuantity _quantity)
  (Getter/Setter|SetQuantityatSlot TargetSlot (Math|Integer|Clamp(Integer) (- _quantity AmountToRemove) 0 (LocalVariables|GetLocalQuantity)))
  (return (Math|Integer|Clamp(Integer) (- AmountToRemove (LocalVariables|GetLocalQuantity)) 0 AmountToRemove)))