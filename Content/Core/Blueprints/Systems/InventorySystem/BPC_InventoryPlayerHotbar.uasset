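; Player hotbar inventory component that selects slots by number key or scroll and equips their items through the character's EquipmentComp.
; Keys apply immediately, while scrolling skips empty slots and debounces with a retriggerable delay that a key press overrides.
; Reselecting the equipped slot unequips it, otherwise a server call equips it.
; When the equipped slot changes, authority re-equips differing items and remotes broadcast selection state.
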(event Custom|SetSelectedSlotIndex
  (params (SelectedSlotIndex :type Integer))
  ;[0.15 0.15 0.15 0.5] Hotbar Scroll
  (bind _output_get (Variables|Default|SetCurrentScrollIndex SelectedSlotIndex))
  (bind _output_get_2 (Variables|Default|SetSelectSlotIndex _output_get))
  (bind _hasitem (CallFunction|TryGetSlotItemDataAsset _output_get_2))
  (Default|CallOnHotbarSlotSelected _hasitem _output_get_2)
  (Variables|Default|SetIsHotkeyPressed true)
  (if (== (Variables|Default|GetEquippedHotbarSlotIndex) (Variables|Default|GetSelectSlotIndex))
    (CallFunction|UnequipCurrentItem)
    ;[0.15 0.15 0.15 0.5] Not Equippable items, highlighted all time
    (bind _itemdataasset (CallFunction|TryGetSlotItemDataAsset (Variables|Default|GetSelectSlotIndex)))
    (bind _itemdata (CallFunction|ResolveSoftItemDataReference _itemdataasset))
    (bind _returnvalue (Class|BPIItemData|IsEquippable(Message) _itemdata))
    (Default|CallOnHotbarSlotSelected (not _returnvalue) (Variables|Default|GetSelectSlotIndex))
    (else
      (CallFunction|TrytoEquipItemSERVER (Variables|Default|GetSelectSlotIndex)))))

(event Custom|UnequipCurrentItem
  ;[0.15 0.15 0.15 0.5] Equip / UnEquip item
  (Variables|Default|SetEquippedHotbarSlotIndex -1)
  (Default|SetEquippedItemSERVER (Variables|/Game/Core/Blueprints/Charactes/BP_PlayerCharacter.BP_PlayerCharacter_C|GetEquipmentComp (Variables|References|GetPlayerCharacter)) "NewEnumerator1"))

(event Custom|TryToEquipItem_SERVER
  (params (SlotIndex :type Integer))
  ;[0.15 0.15 0.15 0.5] Equip / UnEquip item
  (bind _output_get (Variables|Default|SetEquippedHotbarSlotIndex SlotIndex))
  (bind _itemdataasset (CallFunction|TryGetSlotItemDataAsset _output_get))
  (Default|SetEquippedItemSERVER (Variables|/Game/Core/Blueprints/Charactes/BP_PlayerCharacter.BP_PlayerCharacter_C|GetEquipmentComp (Variables|References|GetPlayerCharacter)) "NewEnumerator1" _itemdataasset))

(event Custom|SetSelectedSlotIndexByScroll
  (params (SelectSlotIndex :type Integer))
  ;[0.15 0.15 0.15 0.5] Hotbar Scroll
  (bind _output_get (Variables|Default|SetSelectSlotIndex SelectSlotIndex))
  (Default|CallOnHotbarSlotSelected true _output_get)
  (Variables|Default|SetIsHotkeyPressed false)
  (Utilities|FlowControl|RetriggerableDelay 0.15)
  (if (not (Variables|Default|GetIsHotkeyPressed))
    (if (== (Variables|Default|GetEquippedHotbarSlotIndex) (Variables|Default|GetSelectSlotIndex))
      (CallFunction|UnequipCurrentItem)
      ;[0.15 0.15 0.15 0.5] Not Equippable items, highlighted all time
      (bind _itemdataasset (CallFunction|TryGetSlotItemDataAsset (Variables|Default|GetSelectSlotIndex)))
      (bind _itemdata (CallFunction|ResolveSoftItemDataReference _itemdataasset))
      (bind _returnvalue (Class|BPIItemData|IsEquippable(Message) _itemdata))
      (Default|CallOnHotbarSlotSelected (not _returnvalue) (Variables|Default|GetSelectSlotIndex))
      (else
        (CallFunction|TrytoEquipItemSERVER (Variables|Default|GetSelectSlotIndex))))))

(event Custom|OnSlotChanged_Event
  (params (Slot :type S%20Inventory%20Slot%20Structure))
  ;[0.15 0.15 0.15 0.5] On Slot Changed
  (if (== (Variables|Default|GetEquippedHotbarSlotIndex) (Utilities|Struct|BreakS_InventorySlot Slot))
    (Default|CallOnHotbarSlotSelected (CallFunction|IsSlotNotEmpty Slot) (Variables|Default|GetEquippedHotbarSlotIndex))))

(event Custom|OnSlotChanged_Event_0
  (params (Slot :type S%20Inventory%20Slot%20Structure))
  (bind (_slotindex _itemdataassets) (Utilities|Struct|BreakS_InventorySlot Slot))
  ;[0.15 0.15 0.15 0.5] On Slot Changed
  (bind _itemdataasset (Default|GetEquippedSlotItemDataAsset (Variables|/Game/Core/Blueprints/Charactes/BP_PlayerCharacter.BP_PlayerCharacter_C|GetEquipmentComp (Variables|References|GetPlayerCharacter)) "NewEnumerator1"))
  (if (and (== (Variables|Default|GetEquippedHotbarSlotIndex) _slotindex) (!= _itemdataassets _itemdataasset))
    (CallFunction|TrytoEquipItemSERVER _slotindex)))

(event Input|EnhancedActionEvents|EnhancedInputActionIA_Hotbar_ScrollLeft
  (params (ActionValue :type Boolean) (ElapsedSeconds :type Float%20%28double-precision%29) (TriggeredSeconds :type Float%20%28double-precision%29) (InputAction :type Input%20Action%20Object%20Reference :default "/Game/Core/Data/Input/Actions/Hotbar/IA_Hotbar_ScrollLeft.IA_Hotbar_ScrollLeft"))
  ;[0.15 0.15 0.15 0.5] Hotbar Scroll
  (CallFunction|RotateHotbarSlotIndex -1))

(event Input|EnhancedActionEvents|EnhancedInputActionIA_Hotbar_01
  (params (ActionValue :type Boolean) (ElapsedSeconds :type Float%20%28double-precision%29) (TriggeredSeconds :type Float%20%28double-precision%29) (InputAction :type Input%20Action%20Object%20Reference :default "/Game/Core/Data/Input/Actions/Hotbar/IA_Hotbar_01.IA_Hotbar_01"))
  ;[0.15 0.15 0.15 0.5] Hotbar keys
  (CallFunction|SetSelectedSlotIndex))

(event Input|EnhancedActionEvents|EnhancedInputActionIA_Hotbar_00
  (params (ActionValue :type Boolean) (ElapsedSeconds :type Float%20%28double-precision%29) (TriggeredSeconds :type Float%20%28double-precision%29) (InputAction :type Input%20Action%20Object%20Reference :default "/Game/Core/Data/Input/Actions/Hotbar/IA_Hotbar_00.IA_Hotbar_00"))
  ;[0.15 0.15 0.15 0.5] Hotbar keys
  (CallFunction|SetSelectedSlotIndex 9))

(event Input|EnhancedActionEvents|EnhancedInputActionIA_Hotbar_ScrollRight
  (params (ActionValue :type Boolean) (ElapsedSeconds :type Float%20%28double-precision%29) (TriggeredSeconds :type Float%20%28double-precision%29) (InputAction :type Input%20Action%20Object%20Reference :default "/Game/Core/Data/Input/Actions/Hotbar/IA_Hotbar_ScrollRight.IA_Hotbar_ScrollRight"))
  ;[0.15 0.15 0.15 0.5] Hotbar Scroll
  (CallFunction|RotateHotbarSlotIndex 1))

(event Input|EnhancedActionEvents|EnhancedInputActionIA_Hotbar_02
  (params (ActionValue :type Boolean) (ElapsedSeconds :type Float%20%28double-precision%29) (TriggeredSeconds :type Float%20%28double-precision%29) (InputAction :type Input%20Action%20Object%20Reference :default "/Game/Core/Data/Input/Actions/Hotbar/IA_Hotbar_02.IA_Hotbar_02"))
  ;[0.15 0.15 0.15 0.5] Hotbar keys
  (CallFunction|SetSelectedSlotIndex 1))

(event Input|EnhancedActionEvents|EnhancedInputActionIA_Hotbar_03
  (params (ActionValue :type Boolean) (ElapsedSeconds :type Float%20%28double-precision%29) (TriggeredSeconds :type Float%20%28double-precision%29) (InputAction :type Input%20Action%20Object%20Reference :default "/Game/Core/Data/Input/Actions/Hotbar/IA_Hotbar_03.IA_Hotbar_03"))
  ;[0.15 0.15 0.15 0.5] Hotbar keys
  (CallFunction|SetSelectedSlotIndex 2))

(event Input|EnhancedActionEvents|EnhancedInputActionIA_Hotbar_04
  (params (ActionValue :type Boolean) (ElapsedSeconds :type Float%20%28double-precision%29) (TriggeredSeconds :type Float%20%28double-precision%29) (InputAction :type Input%20Action%20Object%20Reference :default "/Game/Core/Data/Input/Actions/Hotbar/IA_Hotbar_04.IA_Hotbar_04"))
  ;[0.15 0.15 0.15 0.5] Hotbar keys
  (CallFunction|SetSelectedSlotIndex 3))

(event Input|EnhancedActionEvents|EnhancedInputActionIA_Hotbar_05
  (params (ActionValue :type Boolean) (ElapsedSeconds :type Float%20%28double-precision%29) (TriggeredSeconds :type Float%20%28double-precision%29) (InputAction :type Input%20Action%20Object%20Reference :default "/Game/Core/Data/Input/Actions/Hotbar/IA_Hotbar_05.IA_Hotbar_05"))
  ;[0.15 0.15 0.15 0.5] Hotbar keys
  (CallFunction|SetSelectedSlotIndex 4))

(event Input|EnhancedActionEvents|EnhancedInputActionIA_Hotbar_06
  (params (ActionValue :type Boolean) (ElapsedSeconds :type Float%20%28double-precision%29) (TriggeredSeconds :type Float%20%28double-precision%29) (InputAction :type Input%20Action%20Object%20Reference :default "/Game/Core/Data/Input/Actions/Hotbar/IA_Hotbar_06.IA_Hotbar_06"))
  ;[0.15 0.15 0.15 0.5] Hotbar keys
  (CallFunction|SetSelectedSlotIndex 5))

(event Input|EnhancedActionEvents|EnhancedInputActionIA_Hotbar_07
  (params (ActionValue :type Boolean) (ElapsedSeconds :type Float%20%28double-precision%29) (TriggeredSeconds :type Float%20%28double-precision%29) (InputAction :type Input%20Action%20Object%20Reference :default "/Game/Core/Data/Input/Actions/Hotbar/IA_Hotbar_07.IA_Hotbar_07"))
  ;[0.15 0.15 0.15 0.5] Hotbar keys
  (CallFunction|SetSelectedSlotIndex 6))

(event Input|EnhancedActionEvents|EnhancedInputActionIA_Hotbar_08
  (params (ActionValue :type Boolean) (ElapsedSeconds :type Float%20%28double-precision%29) (TriggeredSeconds :type Float%20%28double-precision%29) (InputAction :type Input%20Action%20Object%20Reference :default "/Game/Core/Data/Input/Actions/Hotbar/IA_Hotbar_08.IA_Hotbar_08"))
  ;[0.15 0.15 0.15 0.5] Hotbar keys
  (CallFunction|SetSelectedSlotIndex 7))

(event Input|EnhancedActionEvents|EnhancedInputActionIA_Hotbar_09
  (params (ActionValue :type Boolean) (ElapsedSeconds :type Float%20%28double-precision%29) (TriggeredSeconds :type Float%20%28double-precision%29) (InputAction :type Input%20Action%20Object%20Reference :default "/Game/Core/Data/Input/Actions/Hotbar/IA_Hotbar_09.IA_Hotbar_09"))
  ;[0.15 0.15 0.15 0.5] Hotbar keys
  (CallFunction|SetSelectedSlotIndex 8))

(event EventBeginPlay
  ;[0.15 0.15 0.15 0.5] Begin play
  (|CallParentFunction)
  (bind _playercharacter (Class|BPICharacter|GetBpPlayerCharacter(Message) (Components|GetOwner)))
  (Variables|References|SetPlayerCharacter _playercharacter)
  ;[0.15 0.15 0.15 0.5] On Slot Changed
  (Networking|SwitchHasAuthority
    (:Authority
      (EventDispatchers|AssignOnSlotChanged (delegate Custom|OnSlotChanged_Event_0)))
    (:Remote
      (EventDispatchers|AssignOnSlotChanged (delegate Custom|OnSlotChanged_Event)))))

(event EventEndPlay
  (params (EndPlayReason :type EEndPlayReason%20Enum :default "Destroyed"))
  ;[0.15 0.15 0.15 0.5] Begin play
  (EventDispatchers|UnbindallEventsfromOnHotbarSlotSelected))

(fn TryGetSlotItemDataAsset
  (params (Index :type Integer))
  (bind (_isvalid _slot) (CallFunction|GetSlotatIndex Index))
  (if (and _isvalid (CallFunction|IsSlotEmpty _slot))
    (return false 0)
    (else
      (return true (Utilities|Struct|BreakS_InventorySlot _slot)))))

(fn RotateHotbarSlotIndex
  (params (ScrollDirection :type Integer))
  (Utilities|FlowControl|ForLoopwithBreak 0 (Variables|Default|GetMaxSlotCount) :!label _label
    (:LoopBody
      (bind _output_get (Variables|Default|SetCurrentScrollIndex (+ (Variables|Default|GetCurrentScrollIndex) ScrollDirection)))
      (if (>= _output_get (Variables|Default|GetMaxSlotCount))
        (Variables|Default|SetCurrentScrollIndex 0)
        (elif (< (Variables|Default|GetCurrentScrollIndex) 0)
          (bind _output_get_2 (Variables|Default|SetCurrentScrollIndex (- (Variables|Default|GetMaxSlotCount) 1)))))
      (bind _hasitem (CallFunction|TryGetSlotItemDataAsset _output_get_2))
      (if _hasitem
        (LocalVariables|SetSlotFound true)
        (goto _label Break)))
    (:Completed
      (if (LocalVariables|GetSlotFound)
        (CallFunction|SetSelectedSlotIndexbyScroll (Variables|Default|GetCurrentScrollIndex))))))