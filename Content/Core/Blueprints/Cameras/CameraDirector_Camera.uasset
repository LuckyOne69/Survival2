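; Gameplay camera director that chooses which camera rigs to activate for the character that owns the evaluation context.
; On each run it fetches camera properties from the Character through the GetPropertiesForCameras interface message.
; It activates a rig for Strafe Cam or Aim camera mode, then separately activates another when the stance is Crouch, so crouching can follow a mode activation in the same run.
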(event EventRunCameraDirector
  (params (Params :type Blueprint%20Camera%20Director%20Evaluation%20Params%20Structure%20%28by%20ref%29))
  (bind _returnvalue (Class|BPICharacter|GetPropertiesforCameras(Message) (Class|BlueprintCameraDirectorEvaluator|FindEvaluationContextOwnerActor "/Script/Engine.Character")))
  (Variables|Default|SetProperties%20Camera _returnvalue)
  (Utilities|FlowControl|Sequence
    (:then_0
      (switch Utilities|FlowControl|Switch|SwitchonE_CameraMode (.CameraMode (Utilities|Struct|BreakS_CharacterCameraProperties (Variables|Default|GetProperties%20Camera)))
        (:NewEnumerator0
          (Class|BlueprintCameraDirectorEvaluator|ActivateCameraRig "/Game/Core/Blueprints/Cameras/CABP_TP_Camera.CABP_TP_Camera.CameraRigAsset_0"))
        (:NewEnumerator1
          (Class|BlueprintCameraDirectorEvaluator|ActivateCameraRig "/Game/Core/Blueprints/Cameras/CABP_TP_Camera.CABP_TP_Camera.CameraRigAsset_2"))))
    (:then_1
      (switch Utilities|FlowControl|Switch|SwitchonE_MovementStance (.Stance (Utilities|Struct|BreakS_CharacterCameraProperties (Variables|Default|GetProperties%20Camera)))
        (:NewEnumerator1
          (Class|BlueprintCameraDirectorEvaluator|ActivateCameraRig "/Game/Core/Blueprints/Cameras/CABP_TP_Camera.CABP_TP_Camera.CameraRigAsset_1"))))))