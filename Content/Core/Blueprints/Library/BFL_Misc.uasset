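; Miscellaneous Blueprint function library of shared UI and debug helpers.
; It prints toggleable color-coded error, todo and notice messages, sets widget visibility, places slots into uniform grids by index, and blocking-loads soft icon textures into dynamic materials with an empty-texture fallback.
; Text block styles resolve through the global UI manager from the game instance, falling back to the UI style data asset for editor preview when the manager is invalid.
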(fn SetWidgetVisibility
  (params (Target :type Widget%20Object%20Reference) (Visible :type Boolean))
  (Widget|SetVisibility Target (select Visible "Visible" "Hidden")))

(fn PrintError
  (params (Message :type String) (Data :type String) (Active :type Boolean))
  (if Active
    (Development|PrintString (LocalVariables|Get__WorldContext) (Utilities|String|Append "ERROR:" Message ": " Data) true true "(R=0.848958,G=0.000000,B=0.000000,A=1.000000)" 3e+01)))

(fn PrintTodo
  (params (Message :type String) (Data :type String) (Active :type Boolean))
  (if Active
    (Development|PrintString (LocalVariables|Get__WorldContext) (Utilities|String|Append "TODO:" Message ": " Data) true true "(R=0.848958,G=0.460149,B=0.000000,A=1.000000)" 3e+01)))

(fn PrintNotice
  (params (Message :type String) (Data :type String) (Active :type Boolean))
  (if Active
    (Development|PrintString (LocalVariables|Get__WorldContext) (Utilities|String|Append "NOTICE:" Message ": " Data) true true "(R=0.848958,G=0.838833,B=0.826850,A=1.000000)" 3e+01)))

(fn SetSlotIconSoftObject
  (params (Target :type Image%20Object%20Reference) (Texture2d :type Texture%202D%20Soft%20Object%20Reference))
  (bind _returnvalue (Appearance|GetDynamicMaterial Target :!class /Script/UMG.Image))
  (if (Utilities|IsValidSoftObjectReference Texture2d)
    (bind _returnvalue_2 (Utilities|LoadAssetBlocking Texture2d))
    (bind _astexture_2d (Utilities|Casting|CastToTexture2D _returnvalue_2)
      (:then
        (Rendering|Material|SetTextureParameterValue _returnvalue (LocalVariables|GetTextureParamName) _astexture_2d))
      (:CastFailed
        (BFLMiscPrint|PrintError "Cant cast Icon Soft Object Texture 2D" (Utilities|ToString(SoftObjectReference) Texture2d) true (LocalVariables|Get__WorldContext))))
    (else
      (Rendering|Material|SetTextureParameterValue _returnvalue (LocalVariables|GetTextureParamName) "/Game/Core/Texture/UI/Icons/T_UI_Empty.T_UI_Empty"))))

(fn AddSlottoGrid
  (params (Target :type Uniform%20Grid%20Panel%20Object%20Reference) (SlotIndex :type Integer) (SlotsPerRow :type Integer) (Slot :type User%20Widget%20Object%20Reference%20%28by%20ref%29))
  (bind ___worldcontext (LocalVariables|Get__WorldContext))
  (bind (_row _column) (BFL_MiscWidgetGrid|CalcGridRowColumn SlotIndex SlotsPerRow ___worldcontext))
  (bind _returnvalue (Class|UniformGridPanel|AddChildtoUniformGrid Target Slot _row _column))
  (Layout|GridSlot|SetHorizontalAlignment _returnvalue "HAlign_Center")
  (Layout|GridSlot|SetVerticalAlignment _returnvalue "VAlign_Center"))

(fn CalcGridRowColumn
  (params (Index :type Integer) (PerRow :type Integer))
  (bind _returnvalue (Math|Conversions|ToFloat(Integer) Index))
  (bind _returnvalue_2 (Math|Conversions|ToFloat(Integer) PerRow))
  (bind (_remainder _returnvalue_3) (Math|Float|Division(WholeandRemainder) _returnvalue _returnvalue_2))
  (return _returnvalue_3 (Math|Float|Truncate _remainder)))

(fn GetGlobalUIManager
  (bind _clientservices (Class|BPIGameInstance|GetClientServices(Message) (Game|GetGameInstance (LocalVariables|Get__WorldContext))))
  (return (Variables|/Game/Core/Blueprints/GamePlay/Services/AC_GlobalClientGameServices.AC_GlobalClientGameServices_C|GetBPC_GlobalUIManager _clientservices)))

(fn GetEditorPreviewStyle
  (params (InTextStyle :type E_UI_TextStyle%20Enum :default "NewEnumerator0"))
  (bind _returnvalue (Utilities|LoadAssetBlocking (LocalVariables|GetUIStyleDataAsset)))
  (bind _aspda_ui_style (Utilities|Casting|CastToPDA_UI_Style _returnvalue))
  (bind _textstyleclass (Default|GetTextStyleClassType _aspda_ui_style InTextStyle))
  (return _textstyleclass))

(fn ResolveTextStyle
  (params (InTextStyle :type E_UI_TextStyle%20Enum :default "NewEnumerator0"))
  (bind _globaluimanager (BFLMiscClientGameServices|GetGlobalUIManager))
  (Utilities|IsValid _globaluimanager
    (:Is%20Valid
      (bind _textstyleclass (Default|GetTextStyleClass _globaluimanager InTextStyle))
      (return _textstyleclass))
    (:Is%20Not%20Valid
      (bind _textstyleclass_2 (BFL_MiscWidgetStyle|GetEditorPreviewStyle InTextStyle))
      (return _textstyleclass_2))))

(fn ApplyStyletoTextBlock
  (params (Target :type Common%20Text%20Block%20Object%20Reference) (InTextStyle :type E_UI_TextStyle%20Enum :default "NewEnumerator0"))
  (bind _textstyleclass (BFL_MiscWidgetStyle|ResolveTextStyle InTextStyle))
  (Class|CommonTextBlock|SetStyle Target _textstyleclass))