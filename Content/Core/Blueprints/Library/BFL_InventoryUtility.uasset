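; Blueprint function library of stateless helpers for working with inventory slot structs.
; Empty and contained-item checks test soft object references without loading assets, and slot weight is quantity times item weight.
; Slot creation resolves the soft item data asset to copy ID, weight and default durability.
; The stacking check synchronously loads the target's asset to query stackability and stack size, then compares item IDs.
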(fn IsSlotEmpty
  (params (Slot :type S%20Inventory%20Slot%20Structure))
  (return (not (Utilities|IsValidSoftObjectReference (Utilities|Struct|BreakS_InventorySlot Slot)))))

(fn IsSlotNotEmpty
  (params (Slot :type S%20Inventory%20Slot%20Structure))
  (return (not (BFLInventoryUtility|IsSlotEmpty Slot))))

(fn MAkeItemtoAdd
  (params (ItemDataSoftObject :type PDA%20Item%20Data%20Soft%20Object%20Reference) (Quantity :type Integer))
  (bind _itemdataasset (CallFunction|ResolveSoftItemDataReference ItemDataSoftObject))
  (Utilities|IsValid _itemdataasset
    (:Is%20Valid
      (return (Utilities|Struct|MakeS_InventorySlot (Variables|/Game/Core/Blueprints/PrimaryDataAssets/PDA_ItemData.PDA_ItemData_C|GetItemID _itemdataasset) Quantity 0 ItemDataSoftObject (Default|GetDefaultDurability _itemdataasset) (Default|GetDefaultDurability _itemdataasset) (Variables|/Game/Core/Blueprints/PrimaryDataAssets/PDA_ItemData.PDA_ItemData_C|GetItemWeight _itemdataasset) "(CurrentAmount_7_BA68FF17449E21332020E18D9653B8F2=0.000000,MaxCapacity_8_7843A8614238BB4BBF07F3AC5D545E49=0.000000,ContainedItemDataAsset_9_25FB68404846DEFA53D367991383E637=None)" 0)))
    (:Is%20Not%20Valid
      (Development|PrintString 0 "Can`t resolve ItemDataAsset"))))

(fn GetSlotWeight
  (params (Slot :type S%20Inventory%20Slot%20Structure))
  (bind (_quantity _itemweight) (Utilities|Struct|BreakS_InventorySlot Slot))
  (return (* _quantity _itemweight)))

(fn HasSlotContainedItem
  (params (Slot :type S%20Inventory%20Slot%20Structure))
  (return (Utilities|IsValidSoftObjectReference (Utilities|Struct|BreakS_SlotContainedItem (Utilities|Struct|BreakS_InventorySlot Slot)))))

(fn IsStackeableandHaveSpace
  (params (TargetSlot :type S%20Inventory%20Slot%20Structure%20%28by%20ref%29) (SlotToStack :type S%20Inventory%20Slot%20Structure%20%28by%20ref%29))
  (bind (_itemid _quantity _itemdataassets) (Utilities|Struct|BreakS_InventorySlot TargetSlot))
  (if (BFLInventoryUtility|IsSlotEmpty TargetSlot)
    (return false)
    (else
      (bind _returnvalue (Utilities|LoadAssetBlocking _itemdataassets))
      (bind (_isstackable _stacksize) (Class|BPIItemData|IsItemStackable(Message) _returnvalue))
      (return (Math|Boolean|ANDBoolean _isstackable (< _quantity _stacksize) (== _itemid (Utilities|Struct|BreakS_InventorySlot SlotToStack)))))))