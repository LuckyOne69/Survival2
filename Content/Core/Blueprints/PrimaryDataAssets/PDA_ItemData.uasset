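; Base item data asset that exposes an item's icon, stacking rules and durability through getter functions.
; An item counts as stackable when its stack size exceeds one, and the stack query returns both that flag and the size.
; Durability defaults to none, with the default durability getter meant for child overrides.
; It returns itself as item data, while the resource data getter returns nothing.
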(fn IsStackable
  (return (> (Variables|Default|GetStackSize) 1)))

(fn GetDefaultDurability
  ;[0.15 0.004253 0 0.5] Iverride function - used by children
  (return 0.0))

(fn GetItemData
  (return self))

(fn GetItemIcon
  (return (Variables|Default|GetIcon)))

(fn GetItemResourceData
  (return 0))

(fn IsItemDurabilityBased
  (return false))

(fn IsItemStackable
  (return (CallFunction|IsStackable) (Variables|Default|GetStackSize)))